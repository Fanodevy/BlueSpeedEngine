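; JumpActor_SHADOW is the visual actor for Shadow's jump, with glow and spin-ball materials that reflect his Super Form.
; On BeginPlay it casts its Instigator to ShadowCharacterBlueprint and checks SuperForm.
; When that flag is set, it hides Glow, shows Superglow and applies super spin-ball materials to the static and skeletal meshes.
; The form is read only once, and the actor has no active Tick or overlap logic.
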(event EventBeginPlay
  (bind _asshadow_character_blueprint (Utilities|Casting|CastToShadowCharacterBlueprint (Game|GetInstigator)))
  (if (Variables|/Game/Characters/Shadow/Blueprints/ShadowCharacterBlueprint.ShadowCharacterBlueprint_C|GetSuperForm? _asshadow_character_blueprint)
    (Rendering|SetVisibility (Variables|Default|Getglow) false false)
    (Rendering|SetVisibility (Variables|Default|Getsuperglow) true false)
    (Rendering|Material|SetMaterial (Variables|Default|GetStaticMesh) 0 "/Game/Characters/Sonic/Models/Jump/mat_superspin_ball4.mat_superspin_ball4")
    (Rendering|Material|SetMaterial (Variables|Default|GetSkeletalMesh) 0 "/Game/Characters/Sonic/Models/Jump/mat_superspin_ball5.mat_superspin_ball5")))

(event Collision|EventActorBeginOverlap
  (params (OtherActor :type Actor%20Object%20Reference)))

(event EventTick
  (params (DeltaSeconds :type Float%20%28single-precision%29)))

(fn ConstructionScript)