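; BoostActor_SHADOW is the boost effect actor for Shadow, built from static meshes and energy, stardust and spark effect components.
; On BeginPlay it casts its instigator to ShadowCharacterBlueprint and, if SuperForm is set, swaps the mesh materials and shows the super variants of each effect in place of the normal ones.
; On Hit it spawns a P_PlayerHit emitter at the impact location.
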(event EventBeginPlay
  (bind _asshadow_character_blueprint (Utilities|Casting|CastToShadowCharacterBlueprint (Game|GetInstigator)))
  (if (Variables|/Game/Characters/Shadow/Blueprints/ShadowCharacterBlueprint.ShadowCharacterBlueprint_C|GetSuperForm? _asshadow_character_blueprint)
    (Rendering|Material|SetMaterial (Variables|Default|GetStaticMesh) 0 "/Game/Characters/Sonic/Models/Boost/emt_ch_ssng_yh1_boost_1.emt_ch_ssng_yh1_boost_1")
    (Rendering|Material|SetMaterial (Variables|Default|GetStaticMesh1) 0 "/Game/Characters/Sonic/Models/Boost/emt_ch_ssng_yh1_boost_2.emt_ch_ssng_yh1_boost_2")
    (Rendering|Material|SetMaterial (Variables|Default|GetStaticMesh2) 0 "/Game/Characters/Sonic/Models/Boost/emt_ch_ssng_yh1_boost_2.emt_ch_ssng_yh1_boost_2")
    (Rendering|Material|SetMaterial (Variables|Default|GetStaticMesh3) 0 "/Game/Characters/Sonic/Models/Boost/emt_ch_ssng_yh1_boost_2.emt_ch_ssng_yh1_boost_2")
    (Rendering|Material|SetMaterial (Variables|Default|GetStaticMesh4) 0 "/Game/Characters/Sonic/Models/Boost/emt_ch_ssng_yh1_boost_2.emt_ch_ssng_yh1_boost_2")
    (Rendering|Material|SetMaterial (Variables|Default|GetStaticMesh5) 0 "/Game/Characters/Sonic/Models/Boost/emt_ch_ssng_yh1_boost_2.emt_ch_ssng_yh1_boost_2")
    (Rendering|SetVisibility (Variables|Default|Getenergy) false false)
    (Rendering|SetVisibility (Variables|Default|Getsuperenergy) true false)
    (Rendering|SetVisibility (Variables|Default|Getstardust) false false)
    (Rendering|SetVisibility (Variables|Default|Getsuperstardust) true false)
    (Rendering|SetVisibility (Variables|Default|Getsparks) false false)
    (Rendering|SetVisibility (Variables|Default|Getsupersparks) true false)))

(event Collision|EventActorBeginOverlap
  (params (OtherActor :type Actor%20Object%20Reference)))

(event EventTick
  (params (DeltaSeconds :type Float%20%28single-precision%29)))

(event Collision|EventHit
  (params (MyComp :type Primitive%20Component%20Object%20Reference) (Other :type Actor%20Object%20Reference) (OtherComp :type Primitive%20Component%20Object%20Reference) (bSelfMoved :type Boolean) (HitLocation :type Vector :default "0, 0, 0") (HitNormal :type Vector :default "0, 0, 0") (NormalImpulse :type Vector :default "0, 0, 0") (Hit :type Hit%20Result%20Structure%20%28by%20ref%29))
  (Effects|SpawnEmitteratLocation "/Game/Effects/Particles/P_PlayerHit.P_PlayerHit" HitLocation))

(fn ConstructionScript)