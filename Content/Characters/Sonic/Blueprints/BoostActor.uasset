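; BoostActor is the visual and physical boost effect spawned by Sonic's character.
; On BeginPlay it checks whether its instigator Sonic is in Super Form, then swaps the boost mesh materials and toggles the energy and stardust effects to their super variants.
; On hitting a physics-simulating component, it applies an impulse from its own velocity, attaches spark particles and plays a radial camera shake.
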(event EventBeginPlay
  (bind _assonic_character_blueprint (Utilities|Casting|CastToSonicCharacterBlueprint (Game|GetInstigator)))
  (if (Variables|/Game/Characters/Sonic/Blueprints/SonicCharacterBlueprint.SonicCharacterBlueprint_C|GetSuperForm? _assonic_character_blueprint)
    (Rendering|Material|SetMaterial (Variables|Default|GetStaticMesh) 0 "/Game/Characters/Sonic/Models/Boost/emt_ch_ssng_yh1_boost_1.emt_ch_ssng_yh1_boost_1")
    (Rendering|Material|SetMaterial (Variables|Default|GetStaticMesh1) 0 "/Game/Characters/Sonic/Models/Boost/emt_ch_ssng_yh1_boost_2.emt_ch_ssng_yh1_boost_2")
    (Rendering|Material|SetMaterial (Variables|Default|GetStaticMesh2) 0 "/Game/Characters/Sonic/Models/Boost/emt_ch_ssng_yh1_boost_2.emt_ch_ssng_yh1_boost_2")
    (Rendering|Material|SetMaterial (Variables|Default|GetStaticMesh3) 0 "/Game/Characters/Sonic/Models/Boost/emt_ch_ssng_yh1_boost_2.emt_ch_ssng_yh1_boost_2")
    (Rendering|Material|SetMaterial (Variables|Default|GetStaticMesh4) 0 "/Game/Characters/Sonic/Models/Boost/emt_ch_ssng_yh1_boost_2.emt_ch_ssng_yh1_boost_2")
    (Rendering|Material|SetMaterial (Variables|Default|GetStaticMesh5) 0 "/Game/Characters/Sonic/Models/Boost/emt_ch_ssng_yh1_boost_2.emt_ch_ssng_yh1_boost_2")
    (Rendering|SetVisibility (Variables|Default|Getenergy) false false)
    (Rendering|SetVisibility (Variables|Default|Getsuperenergy) true false)
    (Rendering|SetVisibility (Variables|Default|Getstardust) false false)
    (Rendering|SetVisibility (Variables|Default|GetsuperstardusttStardust) true false)))

(event Collision|EventActorBeginOverlap
  (params (OtherActor :type Actor%20Object%20Reference)))

(event EventTick
  (params (DeltaSeconds :type Float%20%28single-precision%29)))

(event Collision|EventHit
  (params (MyComp :type Primitive%20Component%20Object%20Reference) (Other :type Actor%20Object%20Reference) (OtherComp :type Primitive%20Component%20Object%20Reference) (bSelfMoved :type Boolean) (HitLocation :type Vector :default "0, 0, 0") (HitNormal :type Vector :default "0, 0, 0") (NormalImpulse :type Vector :default "0, 0, 0") (Hit :type Hit%20Result%20Structure%20%28by%20ref%29))
  (bind _returnvalue (Transformation|GetActorLocation))
  (if (Physics|IsSimulatingPhysics OtherComp "None")
    (Physics|AddImpulseatLocation OtherComp (Transformation|GetVelocity) _returnvalue "None")
    (Effects|SpawnEmitterAttached "/Game/Effects/Particles/P_DoubleJumpSparks.P_DoubleJumpSparks" OtherComp "None" HitLocation)
    (Camera|PlayWorldCameraShake "/Game/Blueprints/Camera/Shake/ScreenShakeBoostStomp.ScreenShakeBoostStomp_C" _returnvalue 0.0 1.25e+03)))

(fn ConstructionScript)