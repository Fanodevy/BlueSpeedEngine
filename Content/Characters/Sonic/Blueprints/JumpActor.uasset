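; JumpActor is a Sonic character actor with glow and mesh components, apparently the visual for the jump spin ball.
; On BeginPlay it casts its instigator to SonicCharacterBlueprint and checks the SuperForm flag.
; In Super form it swaps Glow for SuperGlow and applies super spin ball materials to the static and skeletal meshes.
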(event EventBeginPlay
  (bind _assonic_character_blueprint (Utilities|Casting|CastToSonicCharacterBlueprint (Game|GetInstigator)))
  (if (Variables|/Game/Characters/Sonic/Blueprints/SonicCharacterBlueprint.SonicCharacterBlueprint_C|GetSuperForm? _assonic_character_blueprint)
    (Rendering|SetVisibility (Variables|Default|Get%20glow) false false)
    (Rendering|SetVisibility (Variables|Default|Getsuper%20glow) true false)
    (Rendering|Material|SetMaterial (Variables|Default|GetStaticMesh) 0 "/Game/Characters/Sonic/Models/Jump/mat_superspin_ball4.mat_superspin_ball4")
    (Rendering|Material|SetMaterial (Variables|Default|GetSkeletalMesh) 0 "/Game/Characters/Sonic/Models/Jump/mat_superspin_ball5.mat_superspin_ball5")))

(event Collision|EventActorBeginOverlap
  (params (OtherActor :type Actor%20Object%20Reference)))

(event EventTick
  (params (DeltaSeconds :type Float%20%28single-precision%29)))

(fn ConstructionScript)