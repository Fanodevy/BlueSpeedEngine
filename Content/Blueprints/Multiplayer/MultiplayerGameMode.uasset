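; Game mode for local two-player multiplayer that puts Sonic and Shadow into the level as separate players.
; On BeginPlay it spawns Sonic at the first P1Start, then creates a second local player and spawns Shadow at the first P2Start.
; Each controller possesses its character, and its controller ID is passed to CallSetMultiplayer.
; A Removesplitscreen event removes the second player without destroying the pawn.
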(event Custom|Remove%20splitscreen
  (Class|GameplayStatics|RemovePlayer (Game|GetPlayerController 1) false))

(event EventBeginPlay
  (bind _returnvalue (Game|GetPlayerController 1))
  (bind _returnvalue_2 (Game|GetPlayerController 0))
  (Utilities|FlowControl|Sequence
    (:then_0
      (bind _outactors (Actor|GetAllActorsOfClass "/Game/Blueprints/Multiplayer/P1Start.P1Start_C"))
      (bind _returnvalue_3 (Game|SpawnActorfromClass "/Game/Characters/Sonic/Blueprints/SonicCharacterBlueprint.SonicCharacterBlueprint_C" (Transformation|GetActorTransform (Utilities|Array|Get(acopy) _outactors)) "AlwaysSpawn" _returnvalue_2 0))
      (Pawn|Possess _returnvalue_2 _returnvalue_3)
      (Default|CallSetMultiplayer (Class|GameplayStatics|GetPlayerControllerID _returnvalue_2)))
    (:then_1
      (Class|GameplayStatics|CreatePlayer -1)
      (bind _outactors_2 (Actor|GetAllActorsOfClass "/Game/Blueprints/Multiplayer/P2Start.P2Start_C"))
      (bind _returnvalue_4 (Game|SpawnActorfromClass "/Game/Characters/Shadow/Blueprints/ShadowCharacterBlueprint.ShadowCharacterBlueprint_C" (Transformation|GetActorTransform (Utilities|Array|Get(acopy) _outactors_2)) "AlwaysSpawn" _returnvalue 0))
      (Pawn|Possess _returnvalue _returnvalue_4)
      (Default|CallSetMultiplayer (Class|GameplayStatics|GetPlayerControllerID _returnvalue)))))

(fn ConstructionScript)