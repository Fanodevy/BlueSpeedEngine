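; Spike cylinder hazard that damages the Sonic or Shadow characters of the first two players while they overlap its mesh.
; A looping timer started on BeginPlay polls for overlap and applies DamageKnockback as damage, instead of using overlap events.
; A separate player-two path is left over: its damage event is empty, and its logic and multiplayer binding are disconnected.
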(event Custom|Multi
  (params (NewParam :type Integer))
  (Utilities|Time|SetTimerbyFunctionName 0 "Damage P2" 0.01 true))

(event Custom|Damage
  (bind _self self)
  (bind _damageknockback (Variables|Default|GetDamageKnockback))
  (for _index (range 0 1)
    (Utilities|IsValid (Game|GetPlayerCharacter _index)
      (:Is%20Valid
        (if (Collision|IsOverlappingActor (Variables|Default|GetStaticMesh) (Game|GetPlayerCharacter _index) :!class /Script/Engine.PrimitiveComponent)
          (Utilities|FlowControl|Sequence
            (:then_0
              (bind _asshadow_character_blueprint (Utilities|Casting|CastToShadowCharacterBlueprint (Game|GetPlayerCharacter _index)))
              (Game|Damage|ApplyDamage _asshadow_character_blueprint _damageknockback 0 _self))
            (:then_1
              (bind _assonic_character_blueprint (Utilities|Casting|CastToSonicCharacterBlueprint (Game|GetPlayerCharacter _index)))
              (Game|Damage|ApplyDamage _assonic_character_blueprint _damageknockback 0 _self))))))))

(event Custom|Damage%20P2)

(event EventBeginPlay
  (Utilities|Time|SetTimerbyFunctionName 0 "Damage" 0.07 true))

(event Collision|EventActorBeginOverlap
  (params (OtherActor :type Actor%20Object%20Reference)))

(event EventTick
  (params (DeltaSeconds :type Float%20%28single-precision%29)))

(fn ConstructionScript)