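; A ring capsule object that awards rings, score and boost energy to Sonic or Shadow when its effect fires.
; On BeginPlay it binds the Rings event to the inherited effect and plays a timeline that spins the Ring component's world yaw.
; The Rings event passes the configured amounts to AddRing on whichever Shadow and Sonic references are valid.
; Overlap and Tick are unused in this graph.
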(event Custom|Rings
  (bind _ringamount (Variables|Default|GetRingamount))
  (bind _scoreamount (Variables|Default|GetScoreAmount))
  (bind _boostenergyamount (Variables|Default|GetBoostEnergyAmount))
  (bind _shadow (Variables|Default|GetShadow))
  (bind _sonic (Variables|Default|GetSonic))
  (Utilities|FlowControl|Sequence
    (:then_0
      (Utilities|IsValid _shadow
        (:Is%20Valid
          (Default|AddRing _shadow _ringamount _scoreamount _boostenergyamount))))
    (:then_1
      (Utilities|IsValid _sonic
        (:Is%20Valid
          (Default|AddRing _sonic _ringamount _scoreamount _boostenergyamount))))))

(event EventBeginPlay
  (|CallParentFunction)
  (EventDispatchers|BindEventtoEffect (delegate Custom|Rings))
  (bind _newtrack_0 (Timeline|RingSpin Play)
    (:Update
      (Transformation|SetWorldRotation (Variables|Default|GetRing) (Math|Rotator|MakeRotator 0.0 0.0 (* _newtrack_0 -1.8e+02)) false false))))

(event Collision|EventActorBeginOverlap
  (params (OtherActor :type Actor%20Object%20Reference)))

(event EventTick
  (params (DeltaSeconds :type Float%20%28single-precision%29))
  (|CallParentFunction DeltaSeconds) ; This node is disabled and will not be called.\nDrag off pins to build functionality.
)

(event EventDestroyed)

(fn ConstructionScript
  (|CallParentFunction))