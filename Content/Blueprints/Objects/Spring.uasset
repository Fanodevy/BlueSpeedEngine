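; Spring object that launches the Sonic or Shadow character when it overlaps the actor.
; Overlap stops any homing attack, then launches along an actor-rotated SpringPower vector, cancelling a stomp and adding extra upward boost.
; Each launch plays the spring animation, sound and particle effect.
; The construction script stretches an arrow component with SpringPower to show launch strength.
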(event EventBeginPlay)

(event EventTick
  (params (DeltaSeconds :type Float%20%28single-precision%29)))

(event Collision|EventActorBeginOverlap
  (params (OtherActor :type Actor%20Object%20Reference))
  (bind _returnvalue (Transformation|GetActorRotation))
  (bind _returnvalue_2 (Transformation|GetActorForwardVector))
  (bind _returnvalue_3 (Transformation|GetActorRotation))
  (bind _returnvalue_4 (Transformation|GetActorTransform))
  (bind _returnvalue_5 (Transformation|GetActorForwardVector))
  (bind _springpower (Variables|Default|GetSpringPower))
  (bind _springpower_2 (Variables|Default|GetSpringPower))
  (bind _returnvalue_6 (+ _returnvalue_2 (Math|Vector|MakeVector 0.0 0.0 _springpower_2)))
  (bind _returnvalue_7 (+ _returnvalue_5 (Math|Vector|MakeVector 0.0 0.0 _springpower)))
  (bind _returnvalue_8 (Math|Vector|RotateVector _returnvalue_6 _returnvalue))
  (bind _returnvalue_9 (Math|Vector|RotateVector _returnvalue_7 _returnvalue_3))
  (Utilities|FlowControl|Sequence
    (:then_0
      (bind _assonic_character_blueprint (Utilities|Casting|CastToSonicCharacterBlueprint OtherActor))
      (if (Variables|/Game/Characters/Sonic/Blueprints/SonicCharacterBlueprint.SonicCharacterBlueprint_C|GetIsHomingAttacking? _assonic_character_blueprint)
        (Variables|/Game/Characters/Sonic/Blueprints/SonicCharacterBlueprint.SonicCharacterBlueprint_C|SetStopHomingAttack? _assonic_character_blueprint true))
      (if (Variables|/Game/Characters/Sonic/Blueprints/SonicCharacterBlueprint.SonicCharacterBlueprint_C|GetIsStomping? _assonic_character_blueprint)
        (Variables|/Game/Characters/Sonic/Blueprints/SonicCharacterBlueprint.SonicCharacterBlueprint_C|SetIsStomping? _assonic_character_blueprint false)
        (Character|LaunchCharacter _assonic_character_blueprint (+ _returnvalue_8 "0, 0,250.000000") true true)
        (else
          (Character|LaunchCharacter _assonic_character_blueprint _returnvalue_8 true true))))
    (:then_1
      (bind _asshadow_character_blueprint (Utilities|Casting|CastToShadowCharacterBlueprint OtherActor))
      (if (Variables|/Game/Characters/Shadow/Blueprints/ShadowCharacterBlueprint.ShadowCharacterBlueprint_C|GetIsHomingAttacking? _asshadow_character_blueprint)
        (Variables|/Game/Characters/Shadow/Blueprints/ShadowCharacterBlueprint.ShadowCharacterBlueprint_C|SetStopHomingAttack? _asshadow_character_blueprint true))
      (if (Variables|/Game/Characters/Shadow/Blueprints/ShadowCharacterBlueprint.ShadowCharacterBlueprint_C|GetIsStomping? _asshadow_character_blueprint)
        (Variables|/Game/Characters/Shadow/Blueprints/ShadowCharacterBlueprint.ShadowCharacterBlueprint_C|SetIsStomping? _asshadow_character_blueprint false)
        (Character|LaunchCharacter _asshadow_character_blueprint (+ _returnvalue_9 "0, 0,250.000000") true true)
        (else
          (Character|LaunchCharacter _asshadow_character_blueprint _returnvalue_9 true true)))))
  (Components|Animation|PlayAnimation (Variables|Default|GetSkeletalMesh) "/Game/Blueprints/Objects/Assets/Springs/Spring/Spring_Anim.Spring_Anim" false)
  (Audio|PlaySoundatLocation "/Game/Audio/Sound/sound/common/SE_Spring.SE_Spring" (Transformation|GetActorLocation) "0, 0, 0" 1.0 1.0 0.0 "/Game/Audio/Sound/SoundAttenuation.SoundAttenuation" 0 0)
  (Effects|SpawnEmitteratLocation "/Game/Effects/Particles/P_SpringLaunch.P_SpringLaunch" (+ (* (Transformation|GetActorUpVector) 3e+01) (.location _returnvalue_4)) (.rotation _returnvalue_4) (+ (.scale _returnvalue_4) 0.1)))

(fn ConstructionScript
  (Transformation|SetWorldScale3D (Variables|Default|GetArrow) (Math|Vector|MakeVector (/ (/ (Variables|Default|GetSpringPower) 1e+02) 2.0) 1.0 1.0)))