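; Goal ring that marks completion when the Sonic or Shadow character enters its sphere.
; On BeginPlay it loops an attached hum and runs a timeline that records Completiontime, which stops on any actor's overlap.
; The first valid touch fades the hum, plays the goal sound at world origin, and runs three timelines scaling the ring mesh, star and cylinder.
; A delayed DestroyActor is present but unconnected.
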(event OnComponentBeginOverlap(Sphere)
  (params (OverlappedComponent :type Primitive%20Component%20Object%20Reference) (OtherActor :type Actor%20Object%20Reference) (OtherComp :type Primitive%20Component%20Object%20Reference) (OtherBodyIndex :type Integer) (bFromSweep :type Boolean) (SweepResult :type Hit%20Result%20Structure%20%28by%20ref%29))
  (Utilities|FlowControl|Sequence
    (:then_0
      (Utilities|Casting|CastToSonicCharacterBlueprint OtherActor)
      (if (not (Variables|Default|Getcomplete)) :!label _label
        (Audio|Components|Audio|FadeOut (stale EventBeginPlay _returnvalue) 1.0 0.0 "Linear" :!class /Script/Engine.AudioComponent)
        (Audio|PlaySoundatLocation "/Game/Audio/Sound/sound/common/SE_Goalring.SE_Goalring" "0, 0, 0" "0, 0, 0" 1.0 1.0 0.0 0 0 0)
        (Variables|Default|Setcomplete true)
        (Utilities|FlowControl|Sequence
          (:then_0
            (bind _newtrack_0 (Timeline|Timeline_1 PlayFromStart)
              (:Update
                (Transformation|SetWorldScale3D (Variables|Default|GetStaticMesh) (Math|Conversions|ToVector(Float) _newtrack_0)))))
          (:then_1
            (bind _newtrack_0_2 (Timeline|Timeline_2 PlayFromStart)
              (:Update
                (Transformation|SetWorldScale3D (Variables|Default|Getstar) (Math|Conversions|ToVector(Float) _newtrack_0_2)))))
          (:then_2
            (bind _newtrack_0_3 (Timeline|Timeline_3 PlayFromStart)
              (:Update
                (Transformation|SetWorldScale3D (Variables|Default|GetCylinder) (Math|Vector|MakeVector (.X (Math|Vector|BreakVector (Math|Conversions|ToVector(Float) _newtrack_0_3))) (.Y (Math|Vector|BreakVector (Math|Conversions|ToVector(Float) _newtrack_0_3))) 0.0))))))))
    (:then_1
      (Utilities|Casting|CastToShadowCharacterBlueprint OtherActor)
      (goto _label))
    (:then_2
      (bind _newtrack_1 (Timeline|Timeline_0 Stop)
        (:Update
          (Variables|Default|Setcompletiontime _newtrack_1))))))

(event EventBeginPlay
  (Utilities|FlowControl|Sequence
    (:then_0
      (bind _newtrack_1 (Timeline|Timeline_0 Play)
        (:Update
          (Variables|Default|Setcompletiontime _newtrack_1))))
    (:then_1
      (bind _returnvalue (Audio|SpawnSoundAttached "/Game/Audio/Sound/sound/common/SE_Goalring_Lp.SE_Goalring_Lp" (Variables|Default|GetStaticMesh) "None" "0, 0, 0" "0, 0, 0" "KeepRelativeOffset" false 1.0 1.0 0.0 "/Game/Audio/Sound/SoundAttenuation.SoundAttenuation" 0)))))

(fn ConstructionScript)