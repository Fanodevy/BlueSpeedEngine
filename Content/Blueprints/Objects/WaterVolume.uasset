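; Water volume actor that switches Sonic and Shadow characters into water physics and plays water effects.
; Box overlap with a character's BreathCollision attaches breath bubbles and calls WaterPhysicsOn; exit calls WaterPhysicsOff, clears bubbles and can play an exit sound.
; Tick spawns ripples at the surface plane while the player's nose is above water, adding shallow footsteps when moving.
; Local physics and water-running macros are disconnected, superseded by the character Blueprints.
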(event OnComponentBeginOverlap(Box)
  (params (OverlappedComponent :type Primitive%20Component%20Object%20Reference) (OtherActor :type Actor%20Object%20Reference) (OtherComp :type Primitive%20Component%20Object%20Reference) (OtherBodyIndex :type Integer) (bFromSweep :type Boolean) (SweepResult :type Hit%20Result%20Structure%20%28by%20ref%29))
  (Utilities|FlowControl|Sequence
    (:then_0
      (bind _assonic_character_blueprint (Utilities|Casting|CastToSonicCharacterBlueprint OtherActor))
      (Variables|Default|SetSonic _assonic_character_blueprint)
      (if (Class|PrimitiveComponent|IsOverlappingComponent (Variables|/Game/Characters/Sonic/Blueprints/SonicCharacterBlueprint.SonicCharacterBlueprint_C|GetBreathCollision (Variables|Default|GetSonic)) (Variables|Default|GetBox))
        (bind _returnvalue (Effects|SpawnEmitterAttached "/Game/Effects/Particles/P_UWBubbleBeathOut.P_UWBubbleBeathOut" (Variables|/Game/Characters/Sonic/Blueprints/SonicCharacterBlueprint.SonicCharacterBlueprint_C|GetBreathCollision (Variables|Default|GetSonic)) "None" "0, 0, 0" "0, 0, 0" "0.010000,0.010000,0.010000"))
        (Variables|Default|SetBreath _returnvalue)
        (Variables|Default|SetPlayer%20ID (Variables|/Game/Characters/Sonic/Blueprints/SonicCharacterBlueprint.SonicCharacterBlueprint_C|GetOwnerPlayerId (Variables|Default|GetSonic)))
        (Variables|Default|SetNoseInWater? true)
        (Default|WaterPhysicson (Variables|Default|GetSonic))))
    (:then_1
      (bind _asshadow_character_blueprint (Utilities|Casting|CastToShadowCharacterBlueprint OtherActor))
      (Variables|Default|SetShadow _asshadow_character_blueprint)
      (if (Class|PrimitiveComponent|IsOverlappingComponent (Variables|/Game/Characters/Shadow/Blueprints/ShadowCharacterBlueprint.ShadowCharacterBlueprint_C|GetBreathCollision (Variables|Default|GetShadow)) (Variables|Default|GetBox))
        (bind _returnvalue_2 (Effects|SpawnEmitterAttached "/Game/Effects/Particles/P_UWBubbleBeathOut.P_UWBubbleBeathOut" (Variables|/Game/Characters/Shadow/Blueprints/ShadowCharacterBlueprint.ShadowCharacterBlueprint_C|GetBreathCollision (Variables|Default|GetShadow)) "None" "0, 0, 0" "0, 0, 0" "0.010000,0.010000,0.010000"))
        (Variables|Default|SetBreath _returnvalue_2)
        (Variables|Default|SetPlayer%20ID (Variables|/Game/Characters/Shadow/Blueprints/ShadowCharacterBlueprint.ShadowCharacterBlueprint_C|GetOwnerPlayerId (Variables|Default|GetShadow)))
        (Variables|Default|SetNoseInWater? true)
        (Default|WaterPhysicson (Variables|Default|GetShadow))))))

(event OnComponentEndOverlap(Box)
  (params (OverlappedComponent :type Primitive%20Component%20Object%20Reference) (OtherActor :type Actor%20Object%20Reference) (OtherComp :type Primitive%20Component%20Object%20Reference) (OtherBodyIndex :type Integer))
  (bind _breath (Variables|Default|GetBreath))
  (Utilities|FlowControl|Sequence
    (:then_0
      (bind _assonic_character_blueprint (Utilities|Casting|CastToSonicCharacterBlueprint OtherActor))
      (Variables|Default|SetPlayer%20ID (Variables|/Game/Characters/Sonic/Blueprints/SonicCharacterBlueprint.SonicCharacterBlueprint_C|GetOwnerPlayerId _assonic_character_blueprint))
      (bind _output_get (Variables|Default|SetSonic _assonic_character_blueprint))
      (Default|WaterPhysicsOff _output_get)
      (Utilities|FlowControl|Sequence :!label _label
        (:then_0
          (|Out))
        (:then_1
          (|OutofWater))))
    (:then_1
      (bind _asshadow_character_blueprint (Utilities|Casting|CastToShadowCharacterBlueprint OtherActor))
      (Variables|Default|SetPlayer%20ID (Variables|/Game/Characters/Shadow/Blueprints/ShadowCharacterBlueprint.ShadowCharacterBlueprint_C|GetOwnerPlayerId _asshadow_character_blueprint))
      (bind _output_get_2 (Variables|Default|SetShadow _asshadow_character_blueprint))
      (Default|WaterPhysicsOff _output_get_2)
      (goto _label))
    (:then_2
      (Utilities|IsValid _breath
        (:Is%20Valid
          (Components|DestroyComponent _breath))))))

(event EventTick
  (params (DeltaSeconds :type Float%20%28single-precision%29))
  (bind _returnvalue (Game|GetPlayerCharacter 0))
  (bind _returnvalue_2 (Transformation|GetActorLocation _returnvalue))
  (bind (_x _y) (Math|Vector|BreakVector _returnvalue_2))
  (if (Collision|IsOverlappingActor (Variables|Default|GetBox) (Game|GetPlayerCharacter (Variables|Default|GetPlayer%20ID)) :!class /Script/Engine.PrimitiveComponent)
    (Utilities|FlowControl|Sequence
      (:then_1
        (if (Variables|Default|GetNoseInWater?)
          (Utilities|IsValid (stale _returnvalue_3)
            (:Is%20Valid
              (Components|DestroyComponent (stale _returnvalue_3))))
          (elif (> (Math|Vector|VectorLength (Transformation|GetVelocity _returnvalue)) 1.5e+02)
            (Utilities|FlowControl|Sequence
              (:then_0
                (Utilities|FlowControl|Delay 0.05)
                (bind _returnvalue_3 (Effects|SpawnEmitteratLocation "/Game/Effects/Particles/P_WaterRipple.P_WaterRipple" (Math|Vector|MakeVector _x _y (+ (.z (Transformation|GetWorldLocation (Variables|Default|GetPlane))) (Variables|Default|GetPlayerRippleZOffset))) :!label _label)))
              (:then_1
                (Utilities|FlowControl|Delay 0.2)
                (Audio|PlaySoundatLocation "/Game/Audio/Sound/sound/FootStepWaterShallow.FootStepWaterShallow" _returnvalue_2 "0, 0, 0" 1.0 1.0 0.0 "/Game/Audio/Sound/SoundAttenuation.SoundAttenuation" 0 0)))
            (else
              (Utilities|FlowControl|Delay 1.0)
              (goto _label))))))))

(event EventBeginPlay
  (bind _player_id (Variables|Default|GetPlayer%20ID))
  (bind _returnvalue (Game|GetPlayerCharacter _player_id))
  (bind _charactermovement (Variables|/Script/Engine.Character|GetCharacterMovement _returnvalue))
  (Game|SpawnActorfromClass "/Game/Blueprints/Objects/Assets/WaterVolumeSound.WaterVolumeSound_C" (Transformation|GetActorTransform) "Undefined" 0 0)
  (Utilities|FlowControl|Delay 0.1666)
  (Variables|Default|SetDefaultPlayerGravity (Variables|/Script/Engine.CharacterMovementComponent|GetGravityScale _charactermovement))
  (Variables|Default|SetDefaultPlayerTerminalVelocity (Variables|/Script/Engine.PhysicsVolume|GetTerminalVelocity (Class|MovementComponent|GetPhysicsVolume _charactermovement)))
  (Variables|Default|SetDefaultPlayerDeceleration (Variables|/Script/Engine.CharacterMovementComponent|GetBrakingDecelerationFlying _charactermovement))
  (Variables|Default|SetDefaultPlayerAcceleration (Variables|/Script/Engine.CharacterMovementComponent|GetMaxAcceleration _charactermovement)))

(fn ConstructionScript
  (Rendering|Material|SetMaterial (Variables|Default|GetPlane) 0 (Variables|Default|GetWaterMaterial)))