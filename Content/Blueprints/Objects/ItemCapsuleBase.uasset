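; Base item capsule that Sonic or Shadow breaks by attacking or radial damage, triggering CallEffect before destroying itself.
; A downward trace at BeginPlay shows grounded or airborne meshes, disabling body collision when airborne.
; Attacking overlaps reset the player's jump and bounce them unless boosting or flying, with a separate homing-attack bounce and trick.
; Breaking plays sound and particles; enemy projectiles ending overlap also break it.
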(event OnComponentBeginOverlap(Capsule)
  (params (OverlappedComponent :type Primitive%20Component%20Object%20Reference) (OtherActor :type Actor%20Object%20Reference) (OtherComp :type Primitive%20Component%20Object%20Reference) (OtherBodyIndex :type Integer) (bFromSweep :type Boolean) (SweepResult :type Hit%20Result%20Structure%20%28by%20ref%29))
  (Utilities|FlowControl|Sequence
    (:then_0
      (bind _asshadow_character_blueprint (Utilities|Casting|CastToShadowCharacterBlueprint OtherActor))
      (Variables|Default|SetShadow _asshadow_character_blueprint)
      (Utilities|FlowControl|DoOnce false
        (:Completed
          (if (.ReturnValue (|IsAttacking? (|sliding)))
            (Collision|SetCollisionEnabled (Variables|Default|GetBody) "NoCollision")
            (Variables|/Game/Characters/Shadow/Blueprints/ShadowCharacterBlueprint.ShadowCharacterBlueprint_C|SetEnemyJumpReset? (Variables|Default|GetShadow) true)
            (if (or (Variables|/Game/Characters/Shadow/Blueprints/ShadowCharacterBlueprint.ShadowCharacterBlueprint_C|GetIsBoosting? (Variables|Default|GetShadow)) (Class|NavMovementComponent|IsFlying (Variables|/Script/Engine.Character|GetCharacterMovement (Variables|Default|GetShadow))))
              (CallFunction|Broken :!label _label)
              (elif (Variables|/Game/Characters/Shadow/Blueprints/ShadowCharacterBlueprint.ShadowCharacterBlueprint_C|GetIsHomingAttacking? (Variables|Default|GetShadow))
                (Variables|/Game/Characters/Shadow/Blueprints/ShadowCharacterBlueprint.ShadowCharacterBlueprint_C|SetStopHomingAttack? (Variables|Default|GetShadow) true)
                (Character|LaunchCharacter (Variables|Default|GetShadow) (Math|Vector|MakeVector 0.0 0.0 (Variables|Default|GetPlayerBounceOffHoming)) false true)
                (Utilities|FlowControl|Sequence
                  (:then_0
                    (goto _label))
                  (:then_1
                    (Default|PostHomingAttackTrick (Variables|Default|GetShadow))))
                (else
                  (Character|LaunchCharacter (Variables|Default|GetShadow) (Math|Vector|MakeVector 0.0 0.0 (Variables|Default|GetPlayerBounceOff)) false true)
                  (goto _label))))))))
    (:then_1
      (bind _assonic_character_blueprint (Utilities|Casting|CastToSonicCharacterBlueprint OtherActor))
      (Variables|Default|SetSonic _assonic_character_blueprint)
      (Utilities|FlowControl|DoOnce false
        (:Completed
          (if (.ReturnValue (|IsAttacking (|isSliding)))
            (Collision|SetCollisionEnabled (Variables|Default|GetBody) "NoCollision")
            (Variables|/Game/Characters/Sonic/Blueprints/SonicCharacterBlueprint.SonicCharacterBlueprint_C|SetEnemyJumpReset? (Variables|Default|GetSonic) true)
            (if (or (Variables|/Game/Characters/Sonic/Blueprints/SonicCharacterBlueprint.SonicCharacterBlueprint_C|GetIsBoosting? (Variables|Default|GetSonic)) (Class|NavMovementComponent|IsFlying (Variables|/Script/Engine.Character|GetCharacterMovement (Variables|Default|GetSonic))))
              (CallFunction|Broken :!label _label_2)
              (elif (Variables|/Game/Characters/Sonic/Blueprints/SonicCharacterBlueprint.SonicCharacterBlueprint_C|GetIsHomingAttacking? (Variables|Default|GetSonic))
                (Variables|/Game/Characters/Sonic/Blueprints/SonicCharacterBlueprint.SonicCharacterBlueprint_C|SetStopHomingAttack? (Variables|Default|GetSonic) true)
                (Character|LaunchCharacter (Variables|Default|GetSonic) (Math|Vector|MakeVector 0.0 0.0 (Variables|Default|GetPlayerBounceOffHoming)) false true)
                (Utilities|FlowControl|Sequence
                  (:then_0
                    (Default|PostHomingAttackTrick (Variables|Default|GetSonic)))
                  (:then_1
                    (goto _label_2)))
                (else
                  (Character|LaunchCharacter (Variables|Default|GetSonic) (Math|Vector|MakeVector 0.0 0.0 (Variables|Default|GetPlayerBounceOff)) false true)
                  (goto _label_2))))))))))

(event OnComponentEndOverlap(Capsule)
  (params (OverlappedComponent :type Primitive%20Component%20Object%20Reference) (OtherActor :type Actor%20Object%20Reference) (OtherComp :type Primitive%20Component%20Object%20Reference) (OtherBodyIndex :type Integer))
  (bind _shadow (Variables|Default|GetShadow))
  (bind _sonic (Variables|Default|GetSonic))
  (bind _shadow_2 (Variables|Default|GetShadow))
  (Utilities|FlowControl|Delay 0.1)
  (Utilities|FlowControl|Sequence
    (:then_0
      (Utilities|FlowControl|DoOnce false) ; enters at Reset
    )
    (:then_1
      (Utilities|FlowControl|DoOnce false) ; enters at Reset
    )
    (:then_2
      (bind _asenemy_projectile (Utilities|Casting|CastToEnemyProjectile (stale OnComponentBeginOverlap(Capsule) OtherActor)))
      (Actor|DestroyActor _asenemy_projectile)
      (Utilities|FlowControl|Delay 0.1)
      (CallFunction|Broken))))

(event Custom|Broken
  (Audio|PlaySoundatLocation "/Game/Blueprints/Objects/Assets/Itemcapsule/014_Synth_MLT_menu_Item_Capsule.014_Synth_MLT_menu_Item_Capsule" (Transformation|GetActorLocation) "0, 0, 0" 1.0 1.0 0.0 "/Game/Audio/Sound/SoundAttenuation.SoundAttenuation" 0 0)
  (Utilities|FlowControl|Delay 0.06)
  (Effects|SpawnEmitteratLocation "/Game/Effects/Particles/P_Capusle.P_Capusle" (Transformation|GetActorLocation) (Transformation|GetActorRotation) (Transformation|GetActorScale3D))
  (Default|CallEffect)
  (Actor|DestroyActor))

(event EventBeginPlay
  (bind _returnvalue (Transformation|GetActorLocation))
  (bind _returnvalue_2 (Collision|LineTraceByChannel _returnvalue (- _returnvalue "0, 0,120.000000") "TraceTypeQuery1" false 0 "None"))
  (Utilities|FlowControl|Sequence
    (:then_0
      (Rendering|SetVisibility (Variables|Default|GetBaseair) (not _returnvalue_2) false)
      (Rendering|SetVisibility (Variables|Default|Gettopair) (not _returnvalue_2) false)
      (Rendering|SetVisibility (Variables|Default|GetBodyair) (not _returnvalue_2) false))
    (:then_1
      (Rendering|SetVisibility (Variables|Default|GetBase) _returnvalue_2 false)
      (Rendering|SetVisibility (Variables|Default|GetBody) _returnvalue_2 false)
      (Rendering|SetVisibility (Variables|Default|GetTop) _returnvalue_2 false))
    (:then_2
      (if (not _returnvalue_2)
        (Collision|SetCollisionEnabled (Variables|Default|GetBody) "NoCollision")))))

(event Game|Damage|EventRadialDamage
  (params (DamageReceived :type Float%20%28single-precision%29) (DamageType :type Damage%20Type%20Object%20Reference) (Origin :type Vector :default "0, 0, 0") (HitInfo :type Hit%20Result%20Structure%20%28by%20ref%29) (InstigatedBy :type Controller%20Object%20Reference) (DamageCauser :type Actor%20Object%20Reference))
  (Utilities|FlowControl|Sequence
    (:then_0
      (bind _assonic_character_blueprint (Utilities|Casting|CastToSonicCharacterBlueprint DamageCauser))
      (Variables|Default|SetSonic _assonic_character_blueprint))
    (:then_1
      (bind _asshadow_character_blueprint (Utilities|Casting|CastToShadowCharacterBlueprint DamageCauser))
      (Variables|Default|SetShadow _asshadow_character_blueprint)))
  (CallFunction|Broken))

(fn ConstructionScript)