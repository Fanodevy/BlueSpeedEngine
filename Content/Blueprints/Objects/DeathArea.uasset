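; DeathArea is a placeable volume that kills Shadow and Sonic player characters when they touch it.
; Trigger overlap prints a debug message, casts the actor to each character Blueprint and calls its EventOnDeath.
; A successful cast then waits through a shared delay before resetting a DoOnce, though no DoOnce gates the overlap in the visible flow.
; The construction script scales the Trigger proportionally from the Cube's world scale.
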(event OnComponentBeginOverlap(Trigger)
  (params (OverlappedComponent :type Primitive%20Component%20Object%20Reference) (OtherActor :type Actor%20Object%20Reference) (OtherComp :type Primitive%20Component%20Object%20Reference) (OtherBodyIndex :type Integer) (bFromSweep :type Boolean) (SweepResult :type Hit%20Result%20Structure%20%28by%20ref%29))
  (Development|PrintString "touched")
  (Utilities|FlowControl|Sequence
    (:then_0
      (bind _asshadow_character_blueprint (Utilities|Casting|CastToShadowCharacterBlueprint OtherActor))
      (Default|EventonDeath _asshadow_character_blueprint))
    (:then_1
      (bind _assonic_character_blueprint (Utilities|Casting|CastToSonicCharacterBlueprint OtherActor))
      (Default|EventonDeath _assonic_character_blueprint)))
  (Utilities|FlowControl|Delay 5.0)
  (Utilities|FlowControl|DoOnce false) ; enters at Reset
)

(event EventBeginPlay)

(event EventTick
  (params (DeltaSeconds :type Float%20%28single-precision%29)))

(fn ConstructionScript
  (Transformation|SetWorldScale3D (Variables|Default|GetTrigger) (* (Transformation|GetWorldScale (Variables|Default|GetCube)) 1.564)))