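; Trick ramp that launches an overlapping Sonic or Shadow character forward and up, awarding score and boost energy and cancelling any stomp.
; Launch velocity comes from ForwardPower and UpPower rotated to the ramp's orientation, overriding current velocity.
; Both character branches share the sound and particle effects, then disable input for DisableInputForSec.
; The construction script stretches the Arrow component in proportion to ForwardPower.
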(event EventBeginPlay)

(event EventTick
  (params (DeltaSeconds :type Float%20%28single-precision%29)))

(event Collision|EventActorBeginOverlap
  (params (OtherActor :type Actor%20Object%20Reference))
  (bind _returnvalue (Transformation|GetActorLocation))
  (bind _disableinputforsec (Variables|Default|GetDisableInputForSec))
  (Utilities|FlowControl|Sequence
    (:then_0
      (bind _assonic_character_blueprint (Utilities|Casting|CastToSonicCharacterBlueprint OtherActor))
      (Default|AddScore _assonic_character_blueprint 1000 2e+01)
      (Variables|/Game/Characters/Sonic/Blueprints/SonicCharacterBlueprint.SonicCharacterBlueprint_C|SetIsStomping? _assonic_character_blueprint false)
      (Character|LaunchCharacter _assonic_character_blueprint (Math|Vector|RotateVector (+ (Transformation|GetActorForwardVector) (Math|Vector|MakeVector (Variables|Default|GetForwardPower) 0.0 (Variables|Default|GetUpPower))) (Transformation|GetActorRotation)) true true))
    (:then_1
      (bind _asshadow_character_blueprint (Utilities|Casting|CastToShadowCharacterBlueprint OtherActor))
      (Default|AddScore _asshadow_character_blueprint 1000 2e+01)
      (Variables|/Game/Characters/Shadow/Blueprints/ShadowCharacterBlueprint.ShadowCharacterBlueprint_C|SetIsStomping? _asshadow_character_blueprint false)
      (Character|LaunchCharacter _asshadow_character_blueprint (Math|Vector|RotateVector (+ (Transformation|GetActorForwardVector) (Math|Vector|MakeVector (Variables|Default|GetForwardPower) 0.0 (Variables|Default|GetUpPower))) (Transformation|GetActorRotation)) true true)))
  (Audio|PlaySoundatLocation "/Game/Audio/Sound/sound/common/SE_Jumpboard.SE_Jumpboard" _returnvalue "0, 0, 0" 1.0 1.0 0.0 "/Game/Audio/Sound/SoundAttenuation.SoundAttenuation" 0 0)
  (Audio|PlaySoundatLocation "/Game/Audio/Sound/sound/common/SE_Rainbowring.SE_Rainbowring" _returnvalue "0, 0, 0" 1.0 1.0 0.0 "/Game/Audio/Sound/SoundAttenuation.SoundAttenuation" 0 0)
  (Effects|SpawnEmitteratLocation "/Game/Effects/Particles/P_TrickRamp.P_TrickRamp" (Transformation|GetWorldLocation (Variables|Default|GetArrow)) "0, 0, 0" (Transformation|GetActorScale3D))
  (Utilities|FlowControl|Sequence
    (:then_0
      (bind _assonic_character_blueprint_2 (Utilities|Casting|CastToSonicCharacterBlueprint OtherActor))
      (Variables|/Game/Characters/Sonic/Blueprints/SonicCharacterBlueprint.SonicCharacterBlueprint_C|SetForceDisableInput? _assonic_character_blueprint_2 true)
      (Utilities|FlowControl|Delay _disableinputforsec)
      (Variables|/Game/Characters/Sonic/Blueprints/SonicCharacterBlueprint.SonicCharacterBlueprint_C|SetForceDisableInput? _assonic_character_blueprint_2 false))
    (:then_1
      (bind _asshadow_character_blueprint_2 (Utilities|Casting|CastToShadowCharacterBlueprint OtherActor))
      (Variables|/Game/Characters/Shadow/Blueprints/ShadowCharacterBlueprint.ShadowCharacterBlueprint_C|SetForceDisableInput? _asshadow_character_blueprint_2 true)
      (Utilities|FlowControl|Delay _disableinputforsec)
      (Variables|/Game/Characters/Shadow/Blueprints/ShadowCharacterBlueprint.ShadowCharacterBlueprint_C|SetForceDisableInput? _asshadow_character_blueprint_2 false))))

(fn ConstructionScript
  (Transformation|SetWorldScale3D (Variables|Default|GetArrow) (Math|Vector|MakeVector (/ (Variables|Default|GetForwardPower) 1e+02) 1.0 1.0)))