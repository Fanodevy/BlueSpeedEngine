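; Dash panel that launches an overlapping Sonic or Shadow character along its facing, cancelling stomp and setting velocity from DashPanelPower.
; DoOnce gates play the boost sound and ramp effect and snap the character to the panel, resetting shortly after overlap ends.
; Shadow additionally gets attached jet boost particles via JetParticleSpawn.
; The construction script stretches the arrow component to visualize power.
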(event EventBeginPlay)

(event Collision|EventActorEndOverlap
  (params (OtherActor :type Actor%20Object%20Reference))
  (bind _returnvalue (Transformation|GetActorLocation))
  (bind _returnvalue_2 (Transformation|GetActorLocation))
  (bind _sonic (Variables|Default|GetSonic))
  (bind _shadow (Variables|Default|GetShadow))
  (Utilities|FlowControl|RetriggerableDelay 0.2)
  (Utilities|FlowControl|Sequence
    (:then_0
      (Utilities|FlowControl|DoOnce false) ; enters at Reset
    )
    (:then_1
      (Utilities|FlowControl|DoOnce false) ; enters at Reset
    )))

(event EventTick
  (params (DeltaSeconds :type Float%20%28single-precision%29)))

(event Collision|EventActorBeginOverlap
  (params (OtherActor :type Actor%20Object%20Reference))
  (bind _returnvalue (Transformation|GetActorLocation))
  (bind _returnvalue_2 (Transformation|GetActorLocation))
  (Utilities|FlowControl|Sequence
    (:then_0
      (bind _assonic_character_blueprint (Utilities|Casting|CastToSonicCharacterBlueprint OtherActor))
      (Variables|Default|SetSonic _assonic_character_blueprint)
      (Variables|/Game/Characters/Sonic/Blueprints/SonicCharacterBlueprint.SonicCharacterBlueprint_C|SetIsStomping? _assonic_character_blueprint false)
      (Variables|/Script/Engine.MovementComponent|SetVelocity (Variables|/Script/Engine.Character|GetCharacterMovement _assonic_character_blueprint) (Math|Vector|RotateVector (+ (Transformation|GetActorForwardVector) (Math|Vector|MakeVector (Variables|Default|GetDashPanelPower) 0.0 0.0)) (Transformation|GetActorRotation)))
      (Utilities|FlowControl|DoOnce false :!label _label
        (:Completed
          (Audio|PlaySoundatLocation "/Game/Audio/Sound/sound/common/SE_Booster.SE_Booster" _returnvalue_2 "0, 0, 0" 1.0 1.0 0.0 "/Game/Audio/Sound/LoudSoundAttenuation.LoudSoundAttenuation" 0 0)
          (Effects|SpawnEmitteratLocation "/Game/Effects/Particles/P_DashRamp.P_DashRamp" _returnvalue_2 "0, 0, 0" (Transformation|GetActorScale3D)))))
    (:then_1
      (bind _asshadow_character_blueprint (Utilities|Casting|CastToShadowCharacterBlueprint OtherActor))
      (Variables|Default|SetShadow _asshadow_character_blueprint)
      (Variables|/Game/Characters/Shadow/Blueprints/ShadowCharacterBlueprint.ShadowCharacterBlueprint_C|SetIsStomping? _asshadow_character_blueprint false)
      (Variables|/Script/Engine.MovementComponent|SetVelocity (Variables|/Script/Engine.Character|GetCharacterMovement _asshadow_character_blueprint) (Math|Vector|RotateVector (+ (Transformation|GetActorForwardVector) (Math|Vector|MakeVector (Variables|Default|GetDashPanelPower) 0.0 0.0)) (Transformation|GetActorRotation)))
      (|JetParticleSpawn (Variables|/Script/Engine.Character|GetMesh _asshadow_character_blueprint) (Variables|/Script/Engine.Character|GetMesh _asshadow_character_blueprint) (Variables|/Script/Engine.Character|GetMesh _asshadow_character_blueprint)
        (:Exit
          (goto _label))))
    (:then_2
      (Utilities|FlowControl|DoOnce false
        (:Completed
          (Utilities|FlowControl|Sequence
            (:then_0
              (Utilities|IsValid (Variables|Default|GetSonic)
                (:Is%20Valid
                  (Transformation|SetActorLocation (Variables|Default|GetSonic) _returnvalue false false))))
            (:then_1
              (Utilities|IsValid (Variables|Default|GetShadow)
                (:Is%20Valid
                  (Transformation|SetActorLocation (Variables|Default|GetShadow) _returnvalue false false))))))))))

(fn ConstructionScript
  (Transformation|SetWorldScale3D (Variables|Default|GetArrow) (Math|Vector|MakeVector (/ (Variables|Default|GetDashPanelPower) 1e+02) 1.0 1.0)))