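; ElectricShieldCapsule is an item capsule that grants an electric shield to Shadow or Sonic.
; On BeginPlay it runs the parent logic, then binds its GiveElecShield event to the Effect dispatcher.
; When fired, the event checks each character reference for validity, removes that character's existing shields and gives the electric one.
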(event Custom|Give%20Elec%20Shield
  (bind _shadow (Variables|Default|GetShadow))
  (bind _sonic (Variables|Default|GetSonic))
  (Utilities|FlowControl|Sequence
    (:then_0
      (Utilities|IsValid _shadow
        (:Is%20Valid
          (Default|RemoveShield(s) _shadow)
          (Default|GiveElectricShield _shadow))))
    (:then_1
      (Utilities|IsValid _sonic
        (:Is%20Valid
          (Default|RemoveShield(s) _sonic)
          (Default|GiveElectricShield _sonic))))))

(event EventBeginPlay
  (|CallParentFunction)
  (EventDispatchers|BindEventtoEffect (delegate Custom|Give%20Elec%20Shield)))

(fn ConstructionScript
  (|CallParentFunction))