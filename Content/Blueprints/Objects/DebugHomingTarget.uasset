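; DebugHomingTarget is a homing attack target, named as a debug object, that bounces Shadow or Sonic characters upward.
; On sphere overlap, it casts to each character Blueprint and acts only during a homing attack.
; It flags the attack to stop and plays character-specific montages, with Sonic's branch calling two back to back.
; Both branches share one upward launch, applied to player character 0 rather than the overlapping actor.
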(event OnComponentBeginOverlap(Sphere)
  (params (OverlappedComponent :type Primitive%20Component%20Object%20Reference) (OtherActor :type Actor%20Object%20Reference) (OtherComp :type Primitive%20Component%20Object%20Reference) (OtherBodyIndex :type Integer) (bFromSweep :type Boolean) (SweepResult :type Hit%20Result%20Structure%20%28by%20ref%29))
  (Utilities|FlowControl|Sequence
    (:then_0
      (bind _asshadow_character_blueprint (Utilities|Casting|CastToShadowCharacterBlueprint OtherActor))
      (if (Variables|/Game/Characters/Shadow/Blueprints/ShadowCharacterBlueprint.ShadowCharacterBlueprint_C|GetIsHomingAttacking? _asshadow_character_blueprint)
        (Variables|/Game/Characters/Shadow/Blueprints/ShadowCharacterBlueprint.ShadowCharacterBlueprint_C|SetStopHomingAttack? _asshadow_character_blueprint true)
        (Animation|PlayAnimMontage _asshadow_character_blueprint "/Game/Characters/Shadow/AnimAssets/SHHomingTrickMontage.SHHomingTrickMontage" 1.0 "None")
        (Character|LaunchCharacter (Game|GetPlayerCharacter 0) "0, 0,1500.000000" false true :!label _label)))
    (:then_1
      (bind _assonic_character_blueprint (Utilities|Casting|CastToSonicCharacterBlueprint OtherActor))
      (if (Variables|/Game/Characters/Sonic/Blueprints/SonicCharacterBlueprint.SonicCharacterBlueprint_C|GetIsHomingAttacking? _assonic_character_blueprint)
        (Variables|/Game/Characters/Sonic/Blueprints/SonicCharacterBlueprint.SonicCharacterBlueprint_C|SetStopHomingAttack? _assonic_character_blueprint true)
        (Animation|PlayAnimMontage _assonic_character_blueprint "/Game/Characters/Sonic/AnimAssets/HomingTrickMontage1.HomingTrickMontage1" 1.0 "None")
        (Animation|PlayAnimMontage _assonic_character_blueprint "/Game/Characters/Sonic/SuperSonic/anim/HomingAttackMontage.HomingAttackMontage" 1.0 "None")
        (goto _label)))))

(event EventBeginPlay)

(event Collision|EventActorBeginOverlap
  (params (OtherActor :type Actor%20Object%20Reference)))

(event EventTick
  (params (DeltaSeconds :type Float%20%28single-precision%29)))

(fn ConstructionScript)