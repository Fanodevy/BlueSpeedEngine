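; Poppable balloon that bounces Sonic or Shadow on contact, granting score and boost energy when they hit it while attacking.
; Sphere overlap picks the response from the player's move: boosting gives a small lift with possible slow motion, stomping passes through, others bounce, with post-homing tricks where applicable.
; Enemy projectiles also pop it; Pop plays particles and sound, hides the mesh and destroys the actor.
; The construction script sets materials and burst particle from BalloonColor.
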(event OnComponentBeginOverlap(Sphere)
  (params (OverlappedComponent :type Primitive%20Component%20Object%20Reference) (OtherActor :type Actor%20Object%20Reference) (OtherComp :type Primitive%20Component%20Object%20Reference) (OtherBodyIndex :type Integer) (bFromSweep :type Boolean) (SweepResult :type Hit%20Result%20Structure%20%28by%20ref%29))
  (bind _returnvalue (|IsSliding))
  (bind _returnvalue_2 (|IsSliding?))
  (bind (_returnvalue_3 _iskicking_) (|IsAttacking? _returnvalue))
  (bind (_returnvalue_4 _iskicking__2) (|IsAttacking _returnvalue_2))
  (Utilities|FlowControl|Sequence
    (:then_0
      (bind _asshadow_character_blueprint (Utilities|Casting|CastToShadowCharacterBlueprint OtherActor))
      (Variables|Default|SetShadow _asshadow_character_blueprint)
      (Utilities|FlowControl|DoOnce false
        (:Completed
          (if _returnvalue_4
            (if (or _iskicking__2 _returnvalue_2)
              (Animation|PlayAnimMontage (Variables|Default|GetShadow) "/Game/Characters/Shadow/AnimAssets/AirBoostStopMontage.AirBoostStopMontage" 1.0 "None"))
            (Default|AddScore (Variables|Default|GetShadow) (Variables|Default|GetScoreAmount) (Variables|Default|GetBoostEnergyAmount))
            (Variables|/Game/Characters/Shadow/Blueprints/ShadowCharacterBlueprint.ShadowCharacterBlueprint_C|SetEnemyJumpReset? (Variables|Default|GetShadow) true)
            (if (Variables|/Game/Characters/Shadow/Blueprints/ShadowCharacterBlueprint.ShadowCharacterBlueprint_C|GetIsBoosting? (Variables|Default|GetShadow))
              (Character|LaunchCharacter (Variables|Default|GetShadow) "0.0,0.0,100.0" false true)
              (Utilities|FlowControl|Sequence
                (:then_0
                  (CallFunction|Pop))
                (:then_1
                  (if (Variables|/Game/Characters/Shadow/Blueprints/ShadowCharacterBlueprint.ShadowCharacterBlueprint_C|GetCanHomingAttack? (Variables|Default|GetShadow))
                    (Default|SlowMotion (Variables|Default|GetShadow) 0.04))))
              (elif (Variables|/Game/Characters/Shadow/Blueprints/ShadowCharacterBlueprint.ShadowCharacterBlueprint_C|GetIsHomingAttacking? (Variables|Default|GetShadow))
                (Variables|/Game/Characters/Shadow/Blueprints/ShadowCharacterBlueprint.ShadowCharacterBlueprint_C|SetStopHomingAttack? (Variables|Default|GetShadow) true)
                (Character|LaunchCharacter (Variables|Default|GetShadow) (|Shadowlaunch) true true :!label _label)
                (Utilities|FlowControl|Sequence
                  (:then_0
                    (CallFunction|Pop))
                  (:then_1
                    (Default|PostHomingAttackTrick (Variables|Default|GetShadow))))
                (elif (Variables|/Game/Characters/Shadow/Blueprints/ShadowCharacterBlueprint.ShadowCharacterBlueprint_C|GetIsStomping? (Variables|Default|GetShadow))
                  (CallFunction|Pop)
                  (else
                    (Character|LaunchCharacter (Variables|Default|GetShadow) (|Shadowlaunch_2) true true)
                    (CallFunction|Pop)))))
            (else
              (goto _label))))))
    (:then_1
      (bind _assonic_character_blueprint (Utilities|Casting|CastToSonicCharacterBlueprint OtherActor))
      (Variables|Default|SetSonic _assonic_character_blueprint)
      (Utilities|FlowControl|DoOnce false
        (:Completed
          (if _returnvalue_3
            (if (or _iskicking_ _returnvalue)
              (Animation|PlayAnimMontage (Variables|Default|GetSonic) "/Game/Characters/Sonic/AnimAssets/EnemyTrickMontage.EnemyTrickMontage" 1.0 "None"))
            (Default|AddScore (Variables|Default|GetSonic) (Variables|Default|GetScoreAmount) (Variables|Default|GetBoostEnergyAmount))
            (Variables|/Game/Characters/Sonic/Blueprints/SonicCharacterBlueprint.SonicCharacterBlueprint_C|SetEnemyJumpReset? (Variables|Default|GetSonic) true)
            (if (Variables|/Game/Characters/Sonic/Blueprints/SonicCharacterBlueprint.SonicCharacterBlueprint_C|GetIsBoosting? (Variables|Default|GetSonic))
              (Character|LaunchCharacter (Variables|Default|GetSonic) "0, 0,100.000000" false true)
              (Utilities|FlowControl|Sequence
                (:then_0
                  (CallFunction|Pop))
                (:then_1
                  (if (Variables|/Game/Characters/Sonic/Blueprints/SonicCharacterBlueprint.SonicCharacterBlueprint_C|GetCanHomingAttack? (Variables|Default|GetSonic))
                    (Default|SlowMotion (Variables|Default|GetSonic) 0.04))))
              (elif (Variables|/Game/Characters/Sonic/Blueprints/SonicCharacterBlueprint.SonicCharacterBlueprint_C|GetIsHomingAttacking? (Variables|Default|GetSonic))
                (Variables|/Game/Characters/Sonic/Blueprints/SonicCharacterBlueprint.SonicCharacterBlueprint_C|SetStopHomingAttack? (Variables|Default|GetSonic) true)
                (Character|LaunchCharacter (Variables|Default|GetSonic) (|SonicLaunch) true true :!label _label_2)
                (Utilities|FlowControl|Sequence
                  (:then_0
                    (Default|PostHomingAttackTrick (Variables|Default|GetSonic)))
                  (:then_1
                    (CallFunction|Pop)))
                (elif (Variables|/Game/Characters/Sonic/Blueprints/SonicCharacterBlueprint.SonicCharacterBlueprint_C|GetIsStomping? (Variables|Default|GetSonic))
                  (CallFunction|Pop)
                  (else
                    (Character|LaunchCharacter (Variables|Default|GetSonic) (|SonicLaunch_2) true true)
                    (CallFunction|Pop)))))
            (else
              (goto _label_2))))))
    (:then_2
      (Utilities|Casting|CastToEnemyProjectile OtherActor)
      (Effects|SpawnEmitteratLocation "/Game/Effects/Particles/P_BalloonProjectile.P_BalloonProjectile" (Transformation|GetActorLocation))
      (CallFunction|Pop))))

(event OnComponentEndOverlap(Sphere)
  (params (OverlappedComponent :type Primitive%20Component%20Object%20Reference) (OtherActor :type Actor%20Object%20Reference) (OtherComp :type Primitive%20Component%20Object%20Reference) (OtherBodyIndex :type Integer))
  (bind _returnvalue (|IsSliding))
  (bind _returnvalue_2 (|IsSliding?))
  (bind _shadow (Variables|Default|GetShadow))
  (bind _sonic (Variables|Default|GetSonic))
  (bind _shadow_2 (Variables|Default|GetShadow))
  (bind _shadow_3 (Variables|Default|GetShadow))
  (bind _sonic_2 (Variables|Default|GetSonic))
  (bind _sonic_3 (Variables|Default|GetSonic))
  (bind _sonic_4 (Variables|Default|GetSonic))
  (bind (_returnvalue_3 _iskicking_) (|IsAttacking? _returnvalue))
  (bind (_returnvalue_4 _iskicking__2) (|IsAttacking _returnvalue_2))
  (Utilities|FlowControl|Delay 0.2)
  (Utilities|FlowControl|Sequence
    (:then_0
      (Utilities|FlowControl|DoOnce false) ; enters at Reset
    )
    (:then_1
      (Utilities|FlowControl|DoOnce false) ; enters at Reset
    )))

(event Custom|Pop
  (bind _returnvalue (Transformation|GetActorTransform))
  ;[1 1 1] Balloon Pop
  (Effects|SpawnEmitteratLocation (Variables|Default|GetBallonParticle) (.location _returnvalue) (.rotation _returnvalue) (.scale _returnvalue))
  (Audio|SpawnSoundatLocation "/Game/Audio/Sound/sound/common/SE_Balloonexpl.SE_Balloonexpl" (.location _returnvalue) (.rotation _returnvalue) 3.0 1.0 0.0 "/Game/Audio/Sound/SoundAttenuation.SoundAttenuation" 0)
  (Rendering|SetVisibility (Variables|Default|GetSkeletalMesh) false false)
  (Utilities|FlowControl|Delay 0.1)
  (Actor|DestroyActor))

(fn ConstructionScript
  (bind _skeletalmesh (Variables|Default|GetSkeletalMesh))
  (bind _ballooncolor (Variables|Default|GetBalloonColor))
  (Utilities|FlowControl|Sequence
    (:then_0
      (if (Utilities|Enum|Equal(Enum) _ballooncolor "NewEnumerator0")
        (Rendering|Material|SetMaterial _skeletalmesh 0 "/Game/Blueprints/Objects/Assets/Balloon/BalloonBase.BalloonBase")
        (Rendering|Material|SetMaterial _skeletalmesh 1 "/Game/Blueprints/Objects/Assets/Balloon/BalloonBase.BalloonBase")
        (Variables|Default|SetBallonParticle "/Game/Effects/Particles/P_BalloonExp.P_BalloonExp")))
    (:then_1
      (if (Utilities|Enum|Equal(Enum) _ballooncolor "NewEnumerator1")
        (Rendering|Material|SetMaterial _skeletalmesh 0 "/Game/Blueprints/Objects/Assets/Balloon/BalloonBaseBlue.BalloonBaseBlue")
        (Rendering|Material|SetMaterial _skeletalmesh 1 "/Game/Blueprints/Objects/Assets/Balloon/BalloonBaseBlue.BalloonBaseBlue")
        (Variables|Default|SetBallonParticle "/Game/Effects/Particles/P_BalloonExpBlue.P_BalloonExpBlue")))
    (:then_2
      (if (Utilities|Enum|Equal(Enum) _ballooncolor "NewEnumerator2")
        (Rendering|Material|SetMaterial _skeletalmesh 0 "/Game/Blueprints/Objects/Assets/Balloon/BalloonBaseGreen.BalloonBaseGreen")
        (Rendering|Material|SetMaterial _skeletalmesh 1 "/Game/Blueprints/Objects/Assets/Balloon/BalloonBaseGreen.BalloonBaseGreen")
        (Variables|Default|SetBallonParticle "/Game/Effects/Particles/P_BalloonExpGreen.P_BalloonExpGreen")))
    (:then_3
      (if (Utilities|Enum|Equal(Enum) _ballooncolor "NewEnumerator3")
        (Rendering|Material|SetMaterial _skeletalmesh 0 "/Game/Blueprints/Objects/Assets/Balloon/BalloonBaseYellow.BalloonBaseYellow")
        (Rendering|Material|SetMaterial _skeletalmesh 1 "/Game/Blueprints/Objects/Assets/Balloon/BalloonBaseYellow.BalloonBaseYellow")
        (Variables|Default|SetBallonParticle "/Game/Effects/Particles/P_BalloonExpYellow.P_BalloonExpYellow")))))