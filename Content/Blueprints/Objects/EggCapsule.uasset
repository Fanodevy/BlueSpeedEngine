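; Egg Capsule object that damages Sonic or Shadow while granting rings and score.
; On BeginPlay it binds its Damage event to an effect, relying on inherited setup.
; For each valid character reference, Damage spawns a character-specific particle effect, applies knockback damage, calls AddRing with no boost energy, and plays an Eggman spring sound.
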(event Custom|Damage
  (bind _returnvalue (Transformation|GetActorTransform))
  (bind _returnvalue_2 (Transformation|GetActorTransform))
  (bind _self self)
  (bind _shadow (Variables|Default|GetShadow))
  (bind _ringamount (Variables|Default|GetRingAmount))
  (bind _sonic (Variables|Default|GetSonic))
  (bind _damageknockback (Variables|Default|GetDamageKnockback))
  (bind _score_amount (Variables|Default|GetScore%20Amount))
  (Utilities|FlowControl|Sequence
    (:then_0
      (Utilities|IsValid _shadow
        (:Is%20Valid
          (Effects|SpawnEmitteratLocation "/Game/Effects/Particles/P_CapsuleEGG.P_CapsuleEGG" (.location _returnvalue) (.rotation _returnvalue) (.scale _returnvalue))
          (Game|Damage|ApplyDamage _shadow _damageknockback 0 _self)
          (Default|AddRing (Variables|Default|GetShadow) _ringamount _score_amount 0.0))))
    (:then_1
      (Utilities|IsValid _sonic
        (:Is%20Valid
          (Effects|SpawnEmitteratLocation "/Game/Effects/Particles/P_SpringLaunchEGG.P_SpringLaunchEGG" (.location _returnvalue_2) (.rotation _returnvalue_2) (.scale _returnvalue_2))
          (Game|Damage|ApplyDamage _sonic _damageknockback 0 _self)
          (Default|AddRing (Variables|Default|GetSonic) _ringamount _score_amount 0.0)))))
  (Audio|PlaySoundatLocation "/Game/Audio/Sound/sound/common/SE_Eggman_Spring.SE_Eggman_Spring" (Transformation|GetActorLocation) "0, 0, 0" 1.0 1.0 0.0 0 0 0))

(event EventBeginPlay
  (|CallParentFunction)
  (EventDispatchers|BindEventtoEffect (delegate Custom|Damage)))

(fn ConstructionScript
  (|CallParentFunction))