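; Spike panel hazard that pops up and damages Sonic or Shadow characters who come within range.
; A detection sphere, sized in the construction script, records the player ID; if Animated, Tick interpolates the spikes up while that player is inside and down otherwise.
; Paired DoOnce gates play out/in sounds, show a marker above the player and toggle damage, with a short delay on pop-up.
; While damage is enabled, Box overlap applies damage every tick.
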(event OnComponentBeginOverlap(Sphere)
  (params (OverlappedComponent :type Primitive%20Component%20Object%20Reference) (OtherActor :type Actor%20Object%20Reference) (OtherComp :type Primitive%20Component%20Object%20Reference) (OtherBodyIndex :type Integer) (bFromSweep :type Boolean) (SweepResult :type Hit%20Result%20Structure%20%28by%20ref%29))
  (bind _asshadow_character_blueprint (Utilities|Casting|CastToShadowCharacterBlueprint OtherActor)
    (:then
      (Variables|Default|SetPlayer%20ID (Variables|/Game/Characters/Shadow/Blueprints/ShadowCharacterBlueprint.ShadowCharacterBlueprint_C|GetOwnerPlayerId _asshadow_character_blueprint)))
    (:CastFailed
      (bind _assonic_character_blueprint (Utilities|Casting|CastToSonicCharacterBlueprint OtherActor))
      (Variables|Default|SetPlayer%20ID (Variables|/Game/Characters/Sonic/Blueprints/SonicCharacterBlueprint.SonicCharacterBlueprint_C|GetOwnerPlayerId _assonic_character_blueprint)))))

(event EventTick
  (params (DeltaSeconds :type Float%20%28single-precision%29))
  (bind _returnvalue (Utilities|Time|GetWorldDeltaSeconds))
  (bind _returnvalue_2 (Transformation|GetActorLocation))
  (bind _self self)
  (bind _staticmesh (Variables|Default|GetStaticMesh))
  (bind _damageknockback (Variables|Default|GetDamageKnockback))
  (bind _spikepopupspeed (Variables|Default|GetSpikePopupSpeed))
  (bind _player_id (Variables|Default|GetPlayer%20ID))
  (bind _returnvalue_3 (Game|GetPlayerCharacter _player_id))
  (bind _returnvalue_4 (Game|GetPlayerCharacter _player_id))
  (bind _relativelocation (Variables|/Script/Engine.SceneComponent|GetRelativeLocation _staticmesh))
  (Utilities|FlowControl|Sequence
    (:then_0
      (Utilities|IsValid _returnvalue_3
        (:Is%20Valid
          (if (Variables|Default|GetAnimated?)
            (if (Collision|IsOverlappingActor (Variables|Default|GetSphere) _returnvalue_3 :!class /Script/Engine.PrimitiveComponent)
              (Transformation|SetRelativeLocation _staticmesh (Math|Interpolation|VInterpTo _relativelocation "0, 0, 0" _returnvalue _spikepopupspeed) false false)
              (Utilities|FlowControl|Sequence
                (:then_0
                  (Utilities|FlowControl|DoOnce false :!label _label
                    (:Completed
                      (Utilities|FlowControl|Delay (/ (Variables|Default|GetSpikePopupSpeed) 1.7e+02))
                      (Variables|Default|SetCanDamagePlayer? true)
                      (Audio|PlaySoundatLocation "/Game/Audio/Sound/sound/common/SE_Needle_Panel_Out.SE_Needle_Panel_Out" _returnvalue_2 "0, 0, 0" 0.25 2.0 0.0 "/Game/Audio/Sound/SoundAttenuation.SoundAttenuation" 0 0)
                      (Effects|SpawnEmitterAttached "/Game/Effects/Particles/P_ExcPoint.P_ExcPoint" (Variables|/Script/Engine.Character|GetMesh (Game|GetPlayerCharacter (Variables|Default|GetPlayer%20ID))) "None" "0, 0,170.000000" "0, 0, 0" "0.700000,0.700000,0.700000"))))
                (:then_1
                  (goto _label_2 Reset)))
              (else
                (Transformation|SetRelativeLocation _staticmesh (Math|Interpolation|VInterpTo _relativelocation "0, 0,-100.000000" _returnvalue _spikepopupspeed) false false)
                (Utilities|FlowControl|Sequence
                  (:then_0
                    (Utilities|FlowControl|DoOnce false :!label _label_2
                      (:Completed
                        (Variables|Default|SetCanDamagePlayer? false)
                        (Audio|PlaySoundatLocation "/Game/Audio/Sound/sound/common/SE_Needle_Panel_Out.SE_Needle_Panel_Out" _returnvalue_2 "0, 0, 0" 0.25 1.69 0.0 "/Game/Audio/Sound/SoundAttenuation.SoundAttenuation" 0 0))))
                  (:then_1
                    (goto _label Reset)))))))))
    (:then_1
      (if (and (Collision|IsOverlappingActor (Variables|Default|GetBox) _returnvalue_4 :!class /Script/Engine.PrimitiveComponent) (Variables|Default|GetCanDamagePlayer?))
        (Utilities|FlowControl|Sequence
          (:then_0
            (bind _asshadow_character_blueprint (Utilities|Casting|CastToShadowCharacterBlueprint _returnvalue_4))
            (Game|Damage|ApplyDamage _asshadow_character_blueprint _damageknockback 0 _self))
          (:then_1
            (bind _assonic_character_blueprint (Utilities|Casting|CastToSonicCharacterBlueprint _returnvalue_4))
            (Game|Damage|ApplyDamage _assonic_character_blueprint _damageknockback 0 _self)))))))

(fn ConstructionScript
  (Components|Sphere|SetSphereRadius (Variables|Default|GetSphere) (Variables|Default|GetDetectionRadius) true))