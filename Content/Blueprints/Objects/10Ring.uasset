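; Super ring pickup that grants ten rings, score and boost energy to a Sonic or Shadow character that overlaps it.
; Each character is detected by cast and receives the reward through its own Add10Ring call, then both share the sound, destroy and particle burst.
; For Sonic only, a collapsed graph first swaps a shoe material to an emissive one if the ring total is not above zero.
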(event Collision|EventActorBeginOverlap
  (params (OtherActor :type Actor%20Object%20Reference))
  (bind _returnvalue (Transformation|GetActorLocation))
  (Utilities|FlowControl|Sequence
    (:then_0
      (bind _assonic_character_blueprint (Utilities|Casting|CastToSonicCharacterBlueprint OtherActor))
      (Utilities|FlowControl|Sequence
        (:then_0
          (|CollapseGraph_0_2 _assonic_character_blueprint _assonic_character_blueprint))
        (:then_1
          (Default|Add10Ring _assonic_character_blueprint 10 1000 1e+01)
          (Audio|PlaySoundatLocation "/Game/Audio/Sound/sound/common/SE_Superring.SE_Superring" _returnvalue "0, 0, 0" 1.0 1.0 0.0 "/Game/Audio/Sound/SoundAttenuation.SoundAttenuation" 0 0 :!label _label)
          (Actor|DestroyActor)
          (Effects|SpawnEmitteratLocation "/Game/Effects/Particles/P_SRingGet.P_SRingGet" _returnvalue))))
    (:then_1
      (bind _asshadow_character_blueprint (Utilities|Casting|CastToShadowCharacterBlueprint OtherActor))
      (Default|Add10Ring _asshadow_character_blueprint 10 1000 1e+01)
      (goto _label))))

(fn ConstructionScript)