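; RingSpline is a placement actor that lays out a row of Ring actors along a spline.
; The construction script adds AmountOfRings child actor components, spaced evenly by distance from the spline's start to its end.
; Each takes the spline's location converted to actor-local space, but its world-space rotation is used directly as relative rotation.
; The event graph has no runtime logic.
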(event EventBeginPlay)

(event Collision|EventActorBeginOverlap
  (params (OtherActor :type Actor%20Object%20Reference)))

(event EventTick
  (params (DeltaSeconds :type Float%20%28single-precision%29)))

(fn ConstructionScript
  (bind _amountofrings (Variables|Default|GetAmountOfRings))
  (bind _spline (Variables|Default|GetSpline))
  (bind _returnvalue (- _amountofrings 1))
  (for _index (range 0 _returnvalue)
    (bind _returnvalue_2 (AddComponent|AddChildActorComponent false (Math|Transform|MakeTransform (Math|Transform|InverseTransformLocation (Transformation|GetActorTransform) (Spline|GetLocationatDistanceAlongSpline _spline (* _index (/ (Spline|GetSplineLength _spline) (Math|Conversions|ToFloat(Integer) _returnvalue))) "World")) (Spline|GetRotationatDistanceAlongSpline _spline (* _index (/ (Spline|GetSplineLength _spline) (Math|Conversions|ToFloat(Integer) _returnvalue))) "World"))))
    (ChildActorComponent|SetChildActorClass _returnvalue_2 "/Game/Blueprints/Objects/Ring.Ring_C")))