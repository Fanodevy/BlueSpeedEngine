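; Spline-based grind rail that Sonic and Shadow characters snap to and ride, with sound, montages and optional trail.
; Construction builds spline meshes; each tick, collision follows the spline point nearest the player, triggering capture that aligns rotation and projects velocity along the rail.
; Jumping, death, end traces or slow upside-down riding release the rider, while homing attacks on it become forward launches.
; BeginPlay spawns a copy sharing the spline for player 1.
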(event OnComponentBeginOverlap(Collision)
  (params (OverlappedComponent :type Primitive%20Component%20Object%20Reference) (OtherActor :type Actor%20Object%20Reference) (OtherComp :type Primitive%20Component%20Object%20Reference) (OtherBodyIndex :type Integer) (bFromSweep :type Boolean) (SweepResult :type Hit%20Result%20Structure%20%28by%20ref%29))
  (bind _for_player_id (Variables|Default|Getfor%20player%20id))
  (bind _for_player_id_2 (Variables|Default|Getfor%20player%20id))
  (bind _for_player_id_3 (Variables|Default|Getfor%20player%20id))
  (bind _launchforce (Variables|Default|GetLaunchForce))
  (bind _returnvalue (Game|GetPlayerCharacter _for_player_id_2))
  (bind _returnvalue_2 (Game|GetPlayerCharacter _for_player_id))
  (bind _returnvalue_3 (Game|GetPlayerCharacter _for_player_id_3))
  (bind _returnvalue_4 (Transformation|GetActorForwardVector _returnvalue))
  (bind _returnvalue_5 (* _returnvalue_4 _launchforce))
  ;[1 1 1] HomingAttack
  (if (== _returnvalue_3 OtherActor)
    (Utilities|FlowControl|Sequence
      (:then_0
        (bind _asshadow_character_blueprint (Utilities|Casting|CastToShadowCharacterBlueprint _returnvalue_3))
        (Variables|Default|SetShadow _asshadow_character_blueprint)
        (if (Variables|/Game/Characters/Shadow/Blueprints/ShadowCharacterBlueprint.ShadowCharacterBlueprint_C|GetIsHomingAttacking? _asshadow_character_blueprint)
          (if (== (Variables|/Game/Characters/Shadow/Blueprints/ShadowCharacterBlueprint.ShadowCharacterBlueprint_C|GetAttackTarget _asshadow_character_blueprint) self)
            (Variables|/Game/Characters/Shadow/Blueprints/ShadowCharacterBlueprint.ShadowCharacterBlueprint_C|SetStopHomingAttack? (Variables|Default|GetShadow) true)
            (Components|Movement|StopMovementImmediately (Variables|/Script/Engine.Character|GetCharacterMovement (Variables|Default|GetShadow)))
            (Animation|StopAnimMontage (Variables|Default|GetShadow) "/Game/Characters/Shadow/AnimAssets/SHHomingAttack.SHHomingAttack")
            (Utilities|FlowControl|Delay 0.05)
            (Character|LaunchCharacter _returnvalue_2 _returnvalue_5 true true))))
      (:then_1
        (bind _assonic_character_blueprint (Utilities|Casting|CastToSonicCharacterBlueprint _returnvalue_3))
        (Variables|Default|SetSonic _assonic_character_blueprint)
        (if (Variables|/Game/Characters/Sonic/Blueprints/SonicCharacterBlueprint.SonicCharacterBlueprint_C|GetIsHomingAttacking? _assonic_character_blueprint)
          (if (== (Variables|/Game/Characters/Sonic/Blueprints/SonicCharacterBlueprint.SonicCharacterBlueprint_C|GetAttackTarget _assonic_character_blueprint) self)
            (Variables|/Game/Characters/Sonic/Blueprints/SonicCharacterBlueprint.SonicCharacterBlueprint_C|SetStopHomingAttack? (Variables|Default|GetSonic) true)
            (Components|Movement|StopMovementImmediately (Variables|/Script/Engine.Character|GetCharacterMovement (Variables|Default|GetSonic)))
            (Animation|StopAnimMontage (Variables|Default|GetSonic) "/Game/Characters/Sonic/AnimAssets/HomingAttackMontage.HomingAttackMontage")
            (Animation|StopAnimMontage (Variables|Default|GetSonic) "/Game/Characters/Sonic/SuperSonic/anim/HomingAttackMontage.HomingAttackMontage")
            (Utilities|FlowControl|Delay 0.05)
            (Character|LaunchCharacter _returnvalue_2 _returnvalue_5 true true)))))))

(event Custom|RailCatch
  (bind _location (CallFunction|FindClosestGrindPoint))
  (bind _location_2 (CallFunction|FindClosestGrindPoint))
  (bind _for_player_id (Variables|Default|Getfor%20player%20id))
  (bind _createstrace_ (Variables|Default|GetCreatesTrace?))
  (bind _for_player_id_2 (Variables|Default|Getfor%20player%20id))
  (bind _returnvalue (CallFunction|ProjectedPlayerVelocity _location_2))
  (bind _returnvalue_2 (Game|GetPlayerCharacter _for_player_id))
  (bind _returnvalue_3 (Game|GetPlayerCharacter _for_player_id_2))
  (bind _returnvalue_4 (Math|Vector|VectorLength _returnvalue))
  (bind _charactermovement (Variables|/Script/Engine.Character|GetCharacterMovement _returnvalue_2))
  (bind _returnvalue_5 (Class|MovementComponent|GetMaxSpeed _charactermovement))
  (bind _returnvalue_6 (/ _returnvalue_4 _returnvalue_5))
  ;[1 1 1] TickOnCollision
  (bind (_outhit _returnvalue_7) (Class|KismetSystemLibrary|CapsuleTraceSingleforObjects _location (+ _location "0, 0,5.000000") 1e+01 6e+01 (Utilities|Array|MakeArray "ObjectTypeQuery3") false (Variables|Default|GetOverlapingActorsExceptions) "None" true))
  (if _returnvalue_7
    (if (== _returnvalue_3 (.HitActor (Collision|BreakHitResult _outhit)))
      (Utilities|FlowControl|Sequence
        (:then_0
          ;[1 1 1] TickAlways
          (Utilities|FlowControl|DoOnce true) ; enters at Reset
        )
        (:then_1
          (Utilities|FlowControl|Sequence
            (:then_0
              (bind _asshadow_character_blueprint (Utilities|Casting|CastToShadowCharacterBlueprint _returnvalue_3))
              (Variables|Default|SetShadow _asshadow_character_blueprint)
              (Variables|Default|SetBranchSwitcher false)
              (if (or (Variables|/Game/Characters/Shadow/Blueprints/ShadowCharacterBlueprint.ShadowCharacterBlueprint_C|GetJumpPressed? _asshadow_character_blueprint) (Variables|/Game/Characters/Shadow/Blueprints/ShadowCharacterBlueprint.ShadowCharacterBlueprint_C|GetDead? _asshadow_character_blueprint))
                (CallFunction|RailLeave :!label _label)
                (else
                  (Utilities|FlowControl|Sequence
                    (:then_0
                      (if (Variables|Default|GetBranchSwitcher) :!label _label_2
                        (goto _label)
                        (else
                          (bind _reached (CallFunction|TraceBeginEnd))
                          (if _reached
                            (CallFunction|RailLeave :!label _label_3)
                            (elif (and (Variables|Default|GetUpsideDown) (not (Class|MovementComponent|IsExceedingMaxSpeed (Variables|/Script/Engine.Character|GetCharacterMovement (Game|GetPlayerCharacter (Variables|Default|Getfor%20player%20id))) 1.5e+03)))
                              (goto _label_3)
                              (else
                                (Variables|Default|SetOnRail true)
                                (Transformation|SetActorLocationAndRotation _returnvalue_2 _location_2 (CallFunction|PlayerRotation))
                                (CallFunction|SetPlayerVelocity _returnvalue true true false) ; Player target set in func
                                (if (>= _returnvalue_4 2e+01)
                                  _
                                  (else
                                    (Variables|/Script/Engine.MovementComponent|SetVelocity _charactermovement (* (Variables|/Script/Engine.MovementComponent|GetVelocity _charactermovement) 2.0))))
                                (Utilities|IsValid (Variables|Default|GetGrindSoundComp)
                                  (:Is%20Valid
                                    (Audio|Components|Audio|SetPitchMultiplier (Variables|Default|GetGrindSoundComp) (Math|Float|Clamp(Float) _returnvalue_6 0.7 0.9))
                                    (Audio|Components|Audio|SetVolumeMultiplier (Variables|Default|GetGrindSoundComp) (Math|Float|Clamp(Float) (* _returnvalue_6 2.0)) :!class /Script/Engine.AudioComponent))
                                  (:Is%20Not%20Valid
                                    _))
                                (Utilities|FlowControl|DoOnce false
                                  (:Completed
                                    ;[1 1 1] OneTimeEventOnCatch
                                    (Utilities|IsValid (Variables|Default|GetShadow)
                                      (:Is%20Valid
                                        (Default|RailPhysicsON (Variables|Default|GetShadow)))
                                      (:Is%20Not%20Valid
                                        (Utilities|IsValid (Variables|Default|GetSonic)
                                          (:Is%20Valid
                                            (Default|RailPhysicsON (Variables|Default|GetSonic))))))
                                    (Audio|PlaySoundatLocation "/Game/Audio/Sound/sound/common/SE_GrindStart.SE_GrindStart" (Transformation|GetActorLocation (Game|GetPlayerCharacter (Variables|Default|Getfor%20player%20id))) "0, 0, 0" 1.0 1.0 0.2 0 0 0)
                                    (bind _returnvalue_8 (Audio|SpawnSoundAttached (Variables|Default|GetGrindSound) (Variables|/Script/Engine.Character|GetMesh (Game|GetPlayerCharacter (Variables|Default|Getfor%20player%20id))) "None" "0, 0, 0" "0, 0, 0" "KeepRelativeOffset" true 1.5 1.0 0.0 0 0))
                                    (Variables|Default|SetGrindSoundComp _returnvalue_8)
                                    (Utilities|FlowControl|Sequence
                                      (:then_0
                                        (Utilities|IsValid (Variables|Default|GetShadow)
                                          (:Is%20Valid
                                            (Utilities|FlowControl|Sequence
                                              (:then_0
                                                (if _createstrace_
                                                  (Variables|/Game/Characters/Shadow/Blueprints/ShadowCharacterBlueprint.ShadowCharacterBlueprint_C|SetTrace? (Variables|Default|GetShadow) true))
                                                (Variables|/Game/Characters/Shadow/Blueprints/ShadowCharacterBlueprint.ShadowCharacterBlueprint_C|SetIsGrinding? (Variables|Default|GetShadow) true)
                                                (Animation|PlayAnimMontage (Variables|Default|GetShadow) "/Game/Characters/Shadow/AnimAssets/SHGrindLand.SHGrindLand" 1.0 "None"))
                                              (:then_1
                                                (Utilities|IsValid (Variables|/Game/Characters/Shadow/Blueprints/ShadowCharacterBlueprint.ShadowCharacterBlueprint_C|GetJumpBallGround (Variables|Default|GetShadow))
                                                  (:Is%20Valid
                                                    (Actor|DestroyActor (Variables|/Game/Characters/Shadow/Blueprints/ShadowCharacterBlueprint.ShadowCharacterBlueprint_C|GetJumpBallGround (Variables|Default|GetShadow))))))))))
                                      (:then_1
                                        (Utilities|IsValid (Variables|Default|GetSonic)
                                          (:Is%20Valid
                                            (Utilities|FlowControl|Sequence
                                              (:then_0
                                                (if _createstrace_
                                                  (Variables|/Game/Characters/Sonic/Blueprints/SonicCharacterBlueprint.SonicCharacterBlueprint_C|SetTrace? (Variables|Default|GetSonic) true))
                                                (Variables|/Game/Characters/Sonic/Blueprints/SonicCharacterBlueprint.SonicCharacterBlueprint_C|SetIsGrinding? (Variables|Default|GetSonic) true)
                                                (Animation|PlayAnimMontage (Variables|Default|GetSonic) "/Game/Characters/Sonic/AnimAssets/GrindLanding.GrindLanding" 1.0 "None"))
                                              (:then_1
                                                (Utilities|IsValid (Variables|/Game/Characters/Sonic/Blueprints/SonicCharacterBlueprint.SonicCharacterBlueprint_C|GetJumpBallGround (Variables|Default|GetSonic))
                                                  (:Is%20Valid
                                                    (Actor|DestroyActor (Variables|/Game/Characters/Sonic/Blueprints/SonicCharacterBlueprint.SonicCharacterBlueprint_C|GetJumpBallGround (Variables|Default|GetSonic)))))))))))))))))))
                    (:then_1
                      (|shdwstmp))))))
            (:then_1
              (bind _assonic_character_blueprint (Utilities|Casting|CastToSonicCharacterBlueprint _returnvalue_3))
              (bind _output_get (Variables|Default|SetSonic _assonic_character_blueprint))
              (Variables|Default|SetBranchSwitcher false)
              (if (or (Variables|/Game/Characters/Sonic/Blueprints/SonicCharacterBlueprint.SonicCharacterBlueprint_C|GetJumpPressed? _output_get) (Variables|/Game/Characters/Sonic/Blueprints/SonicCharacterBlueprint.SonicCharacterBlueprint_C|GetDead? _output_get))
                (goto _label)
                (else
                  (Utilities|FlowControl|Sequence
                    (:then_0
                      (goto _label_2))
                    (:then_1
                      (|Sonicstmp))))))))))
    (elif (Variables|Default|GetOnRail)
      (Utilities|FlowControl|Sequence
        (:then_0
          (Utilities|IsValid (Variables|Default|GetShadow)
            (:Is%20Valid
              (if (Variables|/Game/Characters/Shadow/Blueprints/ShadowCharacterBlueprint.ShadowCharacterBlueprint_C|GetIsGrinding? (Variables|Default|GetShadow))
                (Variables|Default|SetBranchSwitcher true :!label _label_4)
                (goto _label_2)))))
        (:then_1
          (Utilities|IsValid (Variables|Default|GetSonic)
            (:Is%20Valid
              (if (Variables|/Game/Characters/Sonic/Blueprints/SonicCharacterBlueprint.SonicCharacterBlueprint_C|GetIsGrinding? (Variables|Default|GetSonic))
                (goto _label_4)))))))))

(event Custom|Rail%20Leave
  (bind _shadow (Variables|Default|GetShadow))
  (bind _for_player_id (Variables|Default|Getfor%20player%20id))
  (bind _sonic (Variables|Default|GetSonic))
  (bind _shadow_2 (Variables|Default|GetShadow))
  (bind _sonic_2 (Variables|Default|GetSonic))
  (bind _shadow_3 (Variables|Default|GetShadow))
  (bind _sonic_3 (Variables|Default|GetSonic))
  (bind _createstrace_ (Variables|Default|GetCreatesTrace?))
  (bind _returnvalue (Game|GetPlayerCharacter _for_player_id))
  (bind _jumpballground (Variables|/Game/Characters/Shadow/Blueprints/ShadowCharacterBlueprint.ShadowCharacterBlueprint_C|GetJumpBallGround _shadow_2))
  (bind _jumpballground_2 (Variables|/Game/Characters/Sonic/Blueprints/SonicCharacterBlueprint.SonicCharacterBlueprint_C|GetJumpBallGround _sonic_2))
  ;[1 1 1] Leave
  (Utilities|FlowControl|Sequence
    (:then_0
      (bind _asshadow_character_blueprint (Utilities|Casting|CastToShadowCharacterBlueprint _returnvalue))
      (Variables|/Game/Characters/Shadow/Blueprints/ShadowCharacterBlueprint.ShadowCharacterBlueprint_C|SetIsGrinding? _asshadow_character_blueprint false)
      (Variables|/Game/Characters/Shadow/Blueprints/ShadowCharacterBlueprint.ShadowCharacterBlueprint_C|SetTrace? _asshadow_character_blueprint false)
      (Default|RailPhysicsOFF _asshadow_character_blueprint)
      (Utilities|IsValid (Variables|Default|GetGrindSoundComp) :!label _label
        (:Is%20Valid
          (Audio|Components|Audio|Stop (Variables|Default|GetGrindSoundComp))
          (Components|DestroyComponent (Variables|Default|GetGrindSoundComp)))
        (:Is%20Not%20Valid
          _))
      (Variables|Default|SetGrindSoundComp 0)
      (Utilities|Array|Clear (Variables|Default|GetOverlapingActorsExceptions))
      (Variables|Default|SetOnRail false))
    (:then_1
      (bind _assonic_character_blueprint (Utilities|Casting|CastToSonicCharacterBlueprint _returnvalue))
      (Variables|/Game/Characters/Sonic/Blueprints/SonicCharacterBlueprint.SonicCharacterBlueprint_C|SetIsGrinding? _assonic_character_blueprint false)
      (Variables|/Game/Characters/Sonic/Blueprints/SonicCharacterBlueprint.SonicCharacterBlueprint_C|SetTrace? _assonic_character_blueprint false)
      (Default|RailPhysicsOFF _assonic_character_blueprint)
      (goto _label))
    (:then_2
      ;[1 1 1] TickOnCollision
      (Utilities|FlowControl|DoOnce false) ; enters at Reset
    )))

(event EventBeginPlay
  (Utilities|FlowControl|Sequence
    (:then_0
      (Transformation|SetWorldRotation (Variables|Default|GetCollision) "0, 0, 0" false false))
    (:then_1
      (Utilities|FlowControl|Delay 0.1)
      (if (== (Variables|Default|Getfor%20player%20id) 0)
        (bind _returnvalue (Game|SpawnActorfromClass "GrindRail-Basic_C" (Transformation|GetActorTransform) "AlwaysSpawn" 0 0))
        (Variables|GrindRail-Basic_C|Setfor%20player%20id _returnvalue 1)
        (Variables|GrindRail-Basic_C|SetSpline _returnvalue (Variables|Default|GetSpline))))))

(event EventTick
  (params (DeltaSeconds :type Float%20%28single-precision%29))
  (bind _collision (Variables|Default|GetCollision))
  ;[1 1 1] TickAlways
  (Transformation|SetWorldLocation _collision (CallFunction|FindClosestGrindPoint) false false)
  (bind (_outactors _returnvalue) (Collision|ComponentOverlapActors _collision (Transformation|GetWorldTransform _collision) (Utilities|Array|MakeArray "ObjectTypeQuery3") "/Script/Engine.Character"))
  (if _returnvalue
    (CallFunction|RailCatch)
    (else
      (Utilities|FlowControl|DoOnce true
        (:Completed
          (CallFunction|RailLeave))))))

(fn ConstructionScript
  (bind _spline (Variables|Default|GetSpline))
  (bind _spline_2 (Variables|Default|GetSpline))
  (bind _upvectorarray (Variables|Default|GetUpVectorArray))
  (bind _returnvalue (Utilities|Array|Length _upvectorarray))
  (bind _returnvalue_2 (Spline|GetNumberOfSplinePoints _spline_2))
  (bind _returnvalue_3 (- _returnvalue_2 1))
  (Utilities|FlowControl|Sequence
    (:then_0
      (if (< _returnvalue _returnvalue_3)
        (Utilities|Array|Add _upvectorarray "0,0,1.000000")
        (elif (> _returnvalue _returnvalue_3)
          (Utilities|Array|RemoveIndex _upvectorarray (- _returnvalue 1)))))
    (:then_1
      (for _index (range 0 (- (Spline|GetNumberOfSplinePoints _spline) 2))
        (bind _returnvalue_4 (AddComponent|AddSplineMeshComponent false))
        (Transformation|AttachComponentToComponent _returnvalue_4 _spline "None" "KeepRelative" "KeepRelative" "KeepRelative" true)
        (SplineMesh|SetStartandEnd _returnvalue_4 (.Location (Spline|GetLocationandTangentatSplinePoint _spline _index "Local")) (.Tangent (Spline|GetLocationandTangentatSplinePoint _spline _index "Local")) (.Location (Spline|GetLocationandTangentatSplinePoint _spline (+ _index 1) "Local")) (.Tangent (Spline|GetLocationandTangentatSplinePoint _spline (+ _index 1) "Local")) true :!class /Script/Engine.SplineMeshComponent)
        (Components|StaticMesh|SetStaticMesh _returnvalue_4 (Variables|Default|GetRailMesh))
        (SplineMesh|SetForwardAxis _returnvalue_4 "Y" true)
        (Collision|SetCollisionEnabled _returnvalue_4 "PhysicsOnly")))))

(fn FindClosestGrindPoint
  (bind _for_player_id (Variables|Default|Getfor%20player%20id))
  (bind _spline (Variables|Default|GetSpline))
  (bind _returnvalue (Game|GetPlayerCharacter _for_player_id))
  (bind _returnvalue_2 (Transformation|GetActorLocation _returnvalue))
  (Utilities|IsValid _returnvalue
    (:Is%20Valid
      (return (+ (Spline|FindLocationClosesttoWorldLocation _spline _returnvalue_2 "World") (* (Class|SplineComponent|FindUpVectorClosesttoWorldLocation _spline _returnvalue_2 "World") (Variables|Default|GetCharPositionHeight)))))))

(fn PlayerRotation
  (bind _location (CallFunction|FindClosestGrindPoint))
  (bind _for_player_id (Variables|Default|Getfor%20player%20id))
  (bind _spline (Variables|Default|GetSpline))
  (bind _returnvalue (Game|GetPlayerCharacter _for_player_id))
  (bind _return (CallFunction|NotOppositeDirection _spline))
  (bind _returnvalue_2 (Class|SplineComponent|FindRotationClosesttoWorldLocation _spline _location "World"))
  (bind _roll (Math|Rotator|BreakRotator _returnvalue_2))
  (bind _returnvalue_3 (Math|Rotator|GetRotationXVector _returnvalue_2))
  (bind _returnvalue_4 (Transformation|GetActorLocation _returnvalue))
  (bind _returnvalue_5 (Class|SplineComponent|FindUpVectorClosesttoWorldLocation _spline _returnvalue_4 "World"))
  (bind _returnvalue_6 (>= _roll 9e+01))
  (bind _returnvalue_7 (<= _roll -9e+01))
  (bind _returnvalue_8 (Math|Vector|RotateVectorAroundAxis _returnvalue_3 1.8e+02 _returnvalue_5))
  (bind _returnvalue_9 (or _returnvalue_6 _returnvalue_7))
  (bind _returnvalue_10 (Math|Conversions|RotationFromXVector _returnvalue_8))
  (bind (_roll_2 _pitch _yaw) (Math|Rotator|BreakRotator _returnvalue_10))
  (if _returnvalue_9
    (Variables|Default|SetUpsideDown true)
    (else
      (Variables|Default|SetUpsideDown false)))
  (return (Math|Rotator|SelectRotator (Math|Rotator|SelectRotator _returnvalue_2 (Math|Conversions|RotationFromXVector _returnvalue_8) _return) (Math|Rotator|MakeRotator (- _roll_2 1.8e+02) _pitch _yaw) (not (and (not _return) _returnvalue_9)))))

(fn NotOppositeDirection
  (params (Spline :type Spline%20Component%20Object%20Reference))
  (bind _for_player_id (Variables|Default|Getfor%20player%20id))
  (bind _returnvalue (Game|GetPlayerCharacter _for_player_id))
  (return (>= (Math|Vector|DotProduct (Spline|FindDirectionClosesttoWorldLocation Spline (Transformation|GetActorLocation _returnvalue) "World") (Transformation|GetActorForwardVector _returnvalue)) 0.0)))

(fn SetPlayerVelocity
  (params (Velocity :type Vector) (Horizontal%20Overr :type Boolean) (Vertical%20Overr :type Boolean) (Use%20as%20Multiplier :type Boolean))
  (bind _for_player_id (Variables|Default|Getfor%20player%20id))
  (bind _returnvalue (Game|GetPlayerCharacter _for_player_id))
  (bind _charactermovement (Variables|/Script/Engine.Character|GetCharacterMovement _returnvalue))
  (if Use%20as%20Multiplier
    (Variables|/Script/Engine.MovementComponent|SetVelocity _charactermovement (Math|Vector|MakeVector (* (.x (Variables|/Script/Engine.MovementComponent|GetVelocity _charactermovement)) (.x Velocity)) (* (.y (Variables|/Script/Engine.MovementComponent|GetVelocity _charactermovement)) (.y Velocity)) (* (.z (Variables|/Script/Engine.MovementComponent|GetVelocity _charactermovement)) (.z Velocity))))
    (else
      (Variables|/Script/Engine.MovementComponent|SetVelocity _charactermovement (Math|Vector|MakeVector (Math|Float|SelectFloat (.x Velocity) (+ (.x (Variables|/Script/Engine.MovementComponent|GetVelocity _charactermovement)) (.x Velocity)) Horizontal%20Overr) (Math|Float|SelectFloat (.y Velocity) (+ (.y (Variables|/Script/Engine.MovementComponent|GetVelocity _charactermovement)) (.y Velocity)) Horizontal%20Overr) (Math|Float|SelectFloat (.z Velocity) (+ (.z (Variables|/Script/Engine.MovementComponent|GetVelocity _charactermovement)) (.z Velocity)) Vertical%20Overr))))))

(fn ProjectedPlayerVelocity
  (params (purposed%20direction :type Vector%20%28by%20ref%29))
  (bind _spline (Variables|Default|GetSpline))
  (bind _returnvalue (Spline|FindDirectionClosesttoWorldLocation _spline purposed%20direction "World"))
  (return (Math|Vector|ProjectVectorontoVector (Variables|/Script/Engine.MovementComponent|GetVelocity (Variables|/Script/Engine.Character|GetCharacterMovement (Game|GetPlayerCharacter (Variables|Default|Getfor%20player%20id)))) (Math|Vector|SelectVector (* _returnvalue 1e+03) (* _returnvalue -1e+03) (CallFunction|NotOppositeDirection _spline)))))

(fn TraceBeginEnd
  (bind _array (Utilities|Array|MakeArray "ObjectTypeQuery3"))
  (bind _spline (Variables|Default|GetSpline))
  (bind _returnvalue (Spline|GetLocationatSplinePoint _spline 0 "World"))
  (bind _returnvalue_2 (Spline|GetNumberOfSplinePoints _spline))
  (bind _returnvalue_3 (- _returnvalue_2 -1))
  (bind _returnvalue_4 (Spline|GetLocationatSplinePoint _spline _returnvalue_3 "World"))
  (bind (_outhit _returnvalue_5) (Class|KismetSystemLibrary|CapsuleTraceSingleforObjects _returnvalue_4 (+ _returnvalue_4 "0, 0,5.000000") 1e+01 8e+01 _array false (Variables|Default|GetOverlapingActorsExceptions) "None" true))
  (bind (_outhit_2 _returnvalue_6) (Class|KismetSystemLibrary|CapsuleTraceSingleforObjects _returnvalue (+ _returnvalue "0, 0,5.000000") 1e+01 8e+01 _array false (Variables|Default|GetOverlapingActorsExceptions) "None" true))
  (return (or _returnvalue_5 _returnvalue_6)))