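; A moving platform actor that carries a configurable static mesh along a spline track over a set duration.
; Each tick it advances a clamped time value by a signed direction and moves the mesh to that spline point at constant velocity, leaving rotation untouched.
; At either end it stops or, when looping, reverses with an optional delayed wait.
; The construction script applies mesh, scale, duration, start time and direction, placing the platform on the track.
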(event EventTick
  (params (DeltaSeconds :type Float%20%28single-precision%29))
  (Variables|Default|SetDeltaTime DeltaSeconds)
  (if (Variables|Default|GetbMovePlatform)
    (Utilities|FlowControl|Sequence
      (:then_0
        ;[1 1 1] Platform Movement
        (CallFunction|UpdatePlaformTime)
        (CallFunction|SetPlatformLocationandRotation))
      (:then_1
        (bind _return (CallFunction|EndpointReached))
        (if _return
          (if (Variables|Default|GetbLoop)
            ;[1 1 1] Change Movement Direction
            (Variables|Default|SetPlatformDirection (* (Variables|Default|GetPlatformDirection) -1))
            ;[1 1 1] Endpoint Delay
            (if (Variables|Default|GetbWaitAtEndpoints)
              (Variables|Default|SetbMovePlatform false)
              (Utilities|FlowControl|Delay (Variables|Default|GetPlatformEndpointWaitTime))
              (CallFunction|UpdatePlaformTime)
              (CallFunction|SetPlatformLocationandRotation)
              (Variables|Default|SetbMovePlatform true))
            (else
              (Variables|Default|SetbMovePlatform false))))))))

(fn ConstructionScript
  (Components|StaticMesh|SetStaticMesh (Variables|Default|GetPlatform) (Variables|Default|Getmesh))
  (Transformation|SetWorldScale3D (Variables|Default|GetPlatform) (Variables|Default|GetPlatform%20Scale))
  (Variables|Default|SetPlatformDirection (Variables|Default|GetPlatformStartDirection))
  (Variables|/Script/Engine.SplineComponent|SetDuration (Variables|Default|GetSpline) (Variables|Default|GetTrackDuration))
  (Variables|Default|SetPlatformTime (Variables|Default|GetPlatformStartTime))
  (CallFunction|SetPlatformLocationandRotation))

(fn UpdatePlaformTime
  (Variables|Default|SetcachedPlatformTime (Variables|Default|GetPlatformTime))
  (Variables|Default|SetPlatformTime (Math|Float|Clamp(Float) (+ (* (Variables|Default|GetPlatformDirection) (Variables|Default|GetDeltaTime)) (Variables|Default|GetPlatformTime)) 0.0 (Variables|/Script/Engine.SplineComponent|GetDuration (Variables|Default|GetSpline))))
  (return))

(fn SetPlatformLocationandRotation
  (Transformation|SetWorldLocation (Variables|Default|GetPlatform) (Spline|GetLocationatTime (Variables|Default|GetSpline) (Variables|Default|GetPlatformTime) "World" true) false false))

(fn EndpointReached
  (Math|Integer|CompareInt (Variables|Default|GetPlatformDirection)
    (:>
      (Variables|Default|SetlReturn (Math|Float|NearlyEqual(Float) (Variables|Default|GetPlatformTime) (Variables|/Script/Engine.SplineComponent|GetDuration (Variables|Default|GetSpline)) 1e-06)))
    (:==
      (Development|PrintString "*** Platform Direction equals 0 ***" false))
    (:<
      (Variables|Default|SetlReturn (Math|Float|NearlyEqual(Float) (Variables|Default|GetPlatformTime) 0.0 1e-06))))
  (return (Variables|Default|GetlReturn)))