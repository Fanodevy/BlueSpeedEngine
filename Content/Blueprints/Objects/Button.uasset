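; Floor-switch style button that toggles when a Sonic or Shadow character overlaps its sensor, with a half-second cooldown between presses.
; ButtonActivated updates the mesh glow, light and sound, then ChangeState broadcasts the state and button ID through OnStateChanged.
; It switches off only if CanBeTurnedOff is set; UseDelay forces that, disabling the sensor until a timer re-calls the toggle.
; The construction script applies ButtonColor to light and emissive material.
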(event OnComponentBeginOverlap(SwitchSensor)
  (params (OverlappedComponent :type Primitive%20Component%20Object%20Reference) (OtherActor :type Actor%20Object%20Reference) (OtherComp :type Primitive%20Component%20Object%20Reference) (OtherBodyIndex :type Integer) (bFromSweep :type Boolean) (SweepResult :type Hit%20Result%20Structure%20%28by%20ref%29))
  (if (and (not (Variables|Default|GetInDelay)) (not (Variables|Default|GetCooldown?)))
    (Utilities|FlowControl|Sequence
      (:then_0
        (bind _assonic_character_blueprint (Utilities|Casting|CastToSonicCharacterBlueprint OtherActor)))
      (:then_1
        (Utilities|Casting|CastToShadowCharacterBlueprint OtherActor)))
    (CallFunction|ButtonActivated _assonic_character_blueprint)
    (Variables|Default|SetCooldown? true)
    (Utilities|FlowControl|Delay 0.5)
    (Variables|Default|SetCooldown? false)))

(event Custom|ChangeState
  (params (ButtonState :type Boolean) (ButtonID :type Integer) (Instigator :type Actor%20Object%20Reference))
  (bind _output_get (Variables|Default|SetButton%20On? ButtonState))
  (Default|CallOnStateChanged _output_get ButtonID))

(event EventBeginPlay)

(event Collision|EventActorBeginOverlap
  (params (OtherActor :type Actor%20Object%20Reference)))

(event EventTick
  (params (DeltaSeconds :type Float%20%28single-precision%29)))

(fn ConstructionScript
  (Rendering|Components|Light|SetLightColor (Variables|Default|GetSwitchLight) (Variables|Default|GetButtonColor) true)
  (Rendering|Material|SetVectorParameterValueonMaterials (Variables|Default|GetSwitchMesh) "Emissive" (Math|Conversions|ToVector(LinearColor) (Variables|Default|GetButtonColor)))
  (if (Variables|Default|GetUseDelay)
    (Variables|Default|SetCanBeTurnedOff true)))

(fn ButtonActivated
  (params (Instigator :type Actor%20Object%20Reference))
  (if (not (Variables|Default|GetButton%20On?))
    ;[1 1 1] Button On
    (Rendering|Material|SetScalarParameterValueonMaterials (Variables|Default|GetSwitchMesh) "Brightness" (Variables|Default|GetLightPower))
    (Rendering|Components|Light|SetIntensity (Variables|Default|GetSwitchLight) (Variables|Default|GetLightPower))
    (Audio|PlaySoundatLocation "/Game/Blueprints/Objects/Assets/Buttons/Sounds/TurnOn.TurnOn" (Transformation|GetActorLocation) "0, 0, 0" 1.0 1.0 0.0 0 0 0)
    (bind _output_get (Variables|Default|SetButton%20On? true))
    (CallFunction|ChangeState _output_get (Variables|Default|GetButton%20ID) Instigator)
    (if (Variables|Default|GetUseDelay)
      (Collision|SetCollisionEnabled (Variables|Default|GetSwitchSensor) "NoCollision")
      (Utilities|Time|SetTimerbyFunctionName 0 "Button Activated" (Variables|Default|GetTimerDelay))
      (Variables|Default|SetInDelay true))
    (else
      ;[1 1 1] Button Off
      (if (Variables|Default|GetCanBeTurnedOff)
        (Rendering|Material|SetScalarParameterValueonMaterials (Variables|Default|GetSwitchMesh) "Brightness" 0.0)
        (Rendering|Components|Light|SetIntensity (Variables|Default|GetSwitchLight) 0.0)
        (Audio|PlaySoundatLocation "/Game/Blueprints/Objects/Assets/Buttons/Sounds/TurnOff.TurnOff" (Transformation|GetActorLocation) "0, 0, 0" 1.0 1.0 0.0 0 0 0)
        (bind _output_get_2 (Variables|Default|SetButton%20On? false))
        (CallFunction|ChangeState _output_get_2 (Variables|Default|GetButton%20ID) Instigator)
        (if (Variables|Default|GetUseDelay)
          (Collision|SetCollisionEnabled (Variables|Default|GetSwitchSensor) "QueryOnly")
          (Variables|Default|SetInDelay false))))))