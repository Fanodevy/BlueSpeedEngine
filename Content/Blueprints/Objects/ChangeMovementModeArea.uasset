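; Trigger area that toggles the look-around flag on Sonic and Shadow characters, despite its movement-mode name.
; Entering starts a fast looping timer that enables the flag only while the character is grounded and above SpeedBottomLimit.
; Exiting runs a retriggerable delay into a DoOnce, re-armed on each entry, which stops the timer and clears the flag.
; Debug prints report each state.
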(event OnComponentBeginOverlap(Trigger)
  (params (OverlappedComponent :type Primitive%20Component%20Object%20Reference) (OtherActor :type Actor%20Object%20Reference) (OtherComp :type Primitive%20Component%20Object%20Reference) (OtherBodyIndex :type Integer) (bFromSweep :type Boolean) (SweepResult :type Hit%20Result%20Structure%20%28by%20ref%29))
  (Utilities|FlowControl|Sequence
    (:then_0
      (Utilities|Time|SetTimerbyFunctionName 0 "TimedUpdate" 0.02 true))
    (:then_1
      (Utilities|FlowControl|DoOnce false) ; enters at Reset
    )))

(event OnComponentEndOverlap(Trigger)
  (params (OverlappedComponent :type Primitive%20Component%20Object%20Reference) (OtherActor :type Actor%20Object%20Reference) (OtherComp :type Primitive%20Component%20Object%20Reference) (OtherBodyIndex :type Integer))
  (Utilities|FlowControl|RetriggerableDelay (Variables|Default|GetDelayOnExitBox))
  (Utilities|FlowControl|DoOnce false
    (:Completed
      (Utilities|Time|ClearTimerbyFunctionName 0 "TimedUpdate")
      (Utilities|FlowControl|Sequence
        (:then_0
          (bind _asshadow_character_blueprint (Utilities|Casting|CastToShadowCharacterBlueprint OtherActor))
          (Variables|/Game/Characters/Shadow/Blueprints/ShadowCharacterBlueprint.ShadowCharacterBlueprint_C|SetLook%20Around _asshadow_character_blueprint false))
        (:then_1
          (bind _assonic_character_blueprint (Utilities|Casting|CastToSonicCharacterBlueprint OtherActor))
          (Variables|/Game/Characters/Sonic/Blueprints/SonicCharacterBlueprint.SonicCharacterBlueprint_C|SetLookaround _assonic_character_blueprint false)))
      (Development|PrintString "Reset" true true "(R=0.046639,G=0.000000,B=1.000000,A=1.000000)"))))

(event Custom|TimedUpdate
  (bind _speed_bottom_limit (Variables|Default|Getspeed%20bottom%20limit))
  (Utilities|FlowControl|Sequence
    (:then_0
      (bind _asshadow_character_blueprint (Utilities|Casting|CastToShadowCharacterBlueprint (stale OnComponentBeginOverlap(Trigger) OtherActor)))
      (if (AI|Components|NavMovement|IsFalling (Variables|/Script/Engine.Character|GetCharacterMovement _asshadow_character_blueprint))
        (Variables|/Game/Characters/Shadow/Blueprints/ShadowCharacterBlueprint.ShadowCharacterBlueprint_C|SetLook%20Around _asshadow_character_blueprint false :!label _label)
        (Development|PrintString "Reset" true true "(R=0.065970,G=0.000000,B=1.000000,A=1.000000)" :!label _label_2)
        (elif (not (Class|MovementComponent|IsExceedingMaxSpeed (Variables|/Script/Engine.Character|GetCharacterMovement _asshadow_character_blueprint) _speed_bottom_limit))
          (goto _label)
          (else
            (Variables|/Game/Characters/Shadow/Blueprints/ShadowCharacterBlueprint.ShadowCharacterBlueprint_C|SetLook%20Around _asshadow_character_blueprint true)
            (Development|PrintString "In" true true "(R=0.108034,G=1.000000,B=0.000000,A=1.000000)" :!label _label_3)))))
    (:then_1
      (bind _assonic_character_blueprint (Utilities|Casting|CastToSonicCharacterBlueprint (stale OnComponentBeginOverlap(Trigger) OtherActor)))
      (if (AI|Components|NavMovement|IsFalling (Variables|/Script/Engine.Character|GetCharacterMovement _assonic_character_blueprint))
        _
        (elif (not (Class|MovementComponent|IsExceedingMaxSpeed (Variables|/Script/Engine.Character|GetCharacterMovement _assonic_character_blueprint) _speed_bottom_limit))
          _
          (else
            (Variables|/Game/Characters/Sonic/Blueprints/SonicCharacterBlueprint.SonicCharacterBlueprint_C|SetLookaround _assonic_character_blueprint true)
            (goto _label_3))))
      (Variables|/Game/Characters/Sonic/Blueprints/SonicCharacterBlueprint.SonicCharacterBlueprint_C|SetLookaround _assonic_character_blueprint false)
      (goto _label_2))))

(event EventBeginPlay)

(event Collision|EventActorBeginOverlap
  (params (OtherActor :type Actor%20Object%20Reference)))

(event EventTick
  (params (DeltaSeconds :type Float%20%28single-precision%29)))

(fn ConstructionScript)