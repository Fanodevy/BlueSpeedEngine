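; ShieldCapsule is a capsule object that gives the player characters a normal shield when its effect fires.
; On BeginPlay it runs the parent logic and binds its GiveShield event to the inherited Effect dispatcher.
; GiveShield checks the Shadow and Sonic references separately, and for each valid one removes existing shields before granting the normal shield.
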(event Custom|Give%20Shield
  (bind _shadow (Variables|Default|GetShadow))
  (bind _sonic (Variables|Default|GetSonic))
  (Utilities|FlowControl|Sequence
    (:then_0
      (Utilities|IsValid _shadow
        (:Is%20Valid
          (Default|RemoveShield(s) _shadow)
          (Default|GiveNormalShield _shadow))))
    (:then_1
      (Utilities|IsValid _sonic
        (:Is%20Valid
          (Default|RemoveShield(s) _sonic)
          (Default|GiveNormalShield _sonic))))))

(event EventBeginPlay
  (|CallParentFunction)
  (EventDispatchers|BindEventtoEffect (delegate Custom|Give%20Shield)))

(fn ConstructionScript
  (|CallParentFunction))