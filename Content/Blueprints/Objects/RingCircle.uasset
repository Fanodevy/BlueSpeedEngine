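; RingCircle is a placement Blueprint that lays out Ring actors in a horizontal circle.
; Its construction script loops up to AmountOfRings, adding a child actor component at each evenly stepped yaw angle, offset by Radius around Center.
; Each ring takes the actor's rotation as its relative rotation.
; The event graph holds only empty stubs, so all behavior happens at construction.
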(event EventBeginPlay)

(event Collision|EventActorBeginOverlap
  (params (OtherActor :type Actor%20Object%20Reference)))

(event EventTick
  (params (DeltaSeconds :type Float%20%28single-precision%29)))

(fn ConstructionScript
  (bind _amountofrings (Variables|Default|GetAmountOfRings))
  (for _index (range 0 _amountofrings)
    (bind _returnvalue (AddComponent|AddChildActorComponent false (Math|Transform|MakeTransform (+ (* (Math|Vector|GetForwardVector (Math|Rotator|MakeRotator 0.0 0.0 (Math|Conversions|ToFloat(Integer) (* _index (/ 360 _amountofrings))))) (Variables|Default|GetRadius)) (Variables|Default|GetCenter)) (Transformation|GetActorRotation))))
    (ChildActorComponent|SetChildActorClass _returnvalue "/Game/Blueprints/Objects/Ring.Ring_C")))