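; Eggman-themed spring actor that launches Sonic or Shadow on overlap unless they are homing attacking.
; It stops movement, clears stomping, applies a velocity-change impulse from EggSpringPower along its rotated up axis plus forward vector, and briefly disables input.
; Both character branches share the spring animation, sounds and launch particle.
; The construction script scales an arrow's length by spring power to show launch strength.
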(event EventBeginPlay)

(event EventTick
  (params (DeltaSeconds :type Float%20%28single-precision%29)))

(event Collision|EventActorBeginOverlap
  (params (OtherActor :type Actor%20Object%20Reference))
  (bind _returnvalue (Transformation|GetActorTransform))
  (bind _returnvalue_2 (Transformation|GetActorLocation))
  (bind _inputdelaytime (Variables|Default|GetInputDelayTime))
  (Utilities|FlowControl|Sequence
    (:then_0
      (bind _assonic_character_blueprint (Utilities|Casting|CastToSonicCharacterBlueprint OtherActor))
      (if (not (Variables|/Game/Characters/Sonic/Blueprints/SonicCharacterBlueprint.SonicCharacterBlueprint_C|GetIsHomingAttacking? _assonic_character_blueprint))
        (Utilities|FlowControl|Sequence
          (:then_0
            (Variables|/Game/Characters/Sonic/Blueprints/SonicCharacterBlueprint.SonicCharacterBlueprint_C|SetForceDisableInput? _assonic_character_blueprint true)
            (Utilities|FlowControl|Delay _inputdelaytime)
            (Variables|/Game/Characters/Sonic/Blueprints/SonicCharacterBlueprint.SonicCharacterBlueprint_C|SetForceDisableInput? _assonic_character_blueprint false))
          (:then_1
            (Components|Movement|StopMovementImmediately (Variables|/Script/Engine.Character|GetCharacterMovement _assonic_character_blueprint))
            (Variables|/Game/Characters/Sonic/Blueprints/SonicCharacterBlueprint.SonicCharacterBlueprint_C|SetIsStomping? _assonic_character_blueprint false)
            (Physics|AddImpulse (Variables|/Script/Engine.Character|GetCharacterMovement _assonic_character_blueprint) (Math|Vector|RotateVector (+ (Transformation|GetActorForwardVector) (Math|Vector|MakeVector 0.0 0.0 (Variables|Default|GetEggSpringPower))) (Transformation|GetActorRotation)) true)
            (Components|Animation|SetAnimationMode (Variables|/Script/Engine.Character|GetMesh _assonic_character_blueprint) "AnimationBlueprint")
            (Components|Animation|PlayAnimation (Variables|Default|GetSkeletalMesh) "/Game/Blueprints/Objects/Assets/Springs/EggSpring/EggSpring_Anim.EggSpring_Anim" false :!label _label)
            (Audio|PlaySoundatLocation "/Game/Audio/Sound/sound/common/SE_Spring.SE_Spring" _returnvalue_2 "0, 0, 0" 1.0 1.0 0.0 "/Game/Audio/Sound/SoundAttenuation.SoundAttenuation" 0 0)
            (Audio|PlaySoundatLocation "/Game/Audio/Sound/sound/common/SE_Eggman_Spring.SE_Eggman_Spring" _returnvalue_2 "0, 0, 0" 1.0 1.0 0.0 "/Game/Audio/Sound/SoundAttenuation.SoundAttenuation" 0 0)
            (Effects|SpawnEmitteratLocation "/Game/Effects/Particles/P_SpringLaunchEGG.P_SpringLaunchEGG" (+ (.location _returnvalue) (* (Transformation|GetActorUpVector) 1e+02)) (.rotation _returnvalue) (.scale _returnvalue))))))
    (:then_1
      (bind _asshadow_character_blueprint (Utilities|Casting|CastToShadowCharacterBlueprint OtherActor))
      (if (not (Variables|/Game/Characters/Shadow/Blueprints/ShadowCharacterBlueprint.ShadowCharacterBlueprint_C|GetIsHomingAttacking? _asshadow_character_blueprint))
        (Utilities|FlowControl|Sequence
          (:then_0
            (Components|Movement|StopMovementImmediately (Variables|/Script/Engine.Character|GetCharacterMovement _asshadow_character_blueprint))
            (Variables|/Game/Characters/Shadow/Blueprints/ShadowCharacterBlueprint.ShadowCharacterBlueprint_C|SetIsStomping? _asshadow_character_blueprint false)
            (Physics|AddImpulse (Variables|/Script/Engine.Character|GetCharacterMovement _asshadow_character_blueprint) (Math|Vector|RotateVector (+ (Transformation|GetActorForwardVector) (Math|Vector|MakeVector 0.0 0.0 (Variables|Default|GetEggSpringPower))) (Transformation|GetActorRotation)) true)
            (Components|Animation|SetAnimationMode (Variables|/Script/Engine.Character|GetMesh _asshadow_character_blueprint) "AnimationBlueprint")
            (goto _label))
          (:then_1
            (Variables|/Game/Characters/Shadow/Blueprints/ShadowCharacterBlueprint.ShadowCharacterBlueprint_C|SetForceDisableInput? _asshadow_character_blueprint true)
            (Utilities|FlowControl|Delay _inputdelaytime)
            (Variables|/Game/Characters/Shadow/Blueprints/ShadowCharacterBlueprint.ShadowCharacterBlueprint_C|SetForceDisableInput? _asshadow_character_blueprint false)))))))

(fn ConstructionScript
  (Transformation|SetWorldScale3D (Variables|Default|GetArrow) (Math|Vector|MakeVector (/ (/ (Variables|Default|GetEggSpringPower) 1e+02) 3.0) 1.0 1.0)))