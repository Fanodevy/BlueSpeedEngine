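; Rainbow dash ring that snaps an overlapping Sonic or Shadow character to its center and launches them along its facing by DashRingPower.
; The first pass triggers a trick voice, score, boost energy and rainbow effects, then swaps the mesh to a normal hoop.
; Once normal, launches play standard effects and briefly lock input, scaled by the character's time dilation.
; The construction script stretches an arrow to show launch power.
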(event EventBeginPlay)

(event EventTick
  (params (DeltaSeconds :type Float%20%28single-precision%29)))

(event Collision|EventActorBeginOverlap
  (params (OtherActor :type Actor%20Object%20Reference))
  (bind _returnvalue (Transformation|GetActorTransform))
  (bind _returnvalue_2 (Transformation|GetActorLocation))
  (bind _returnvalue_3 (Transformation|GetActorTransform))
  (bind _skeletalmesh (Variables|Default|GetSkeletalMesh))
  (bind _inputdelay (Variables|Default|GetInputDelay))
  (Utilities|FlowControl|Sequence
    (:then_0
      (bind _assonic_character_blueprint (Utilities|Casting|CastToSonicCharacterBlueprint OtherActor))
      (Utilities|FlowControl|Sequence
        (:then_0
          (Variables|/Game/Characters/Sonic/Blueprints/SonicCharacterBlueprint.SonicCharacterBlueprint_C|SetIsStomping? _assonic_character_blueprint false)
          (Transformation|SetWorldLocation (Variables|/Script/Engine.Actor|GetRootComponent _assonic_character_blueprint) _returnvalue_2 false false)
          (Character|LaunchCharacter _assonic_character_blueprint (Math|Vector|RotateVector (+ (Transformation|GetActorForwardVector) (Math|Vector|MakeVector (Variables|Default|GetDashRingPower) 0.0 0.0)) (Transformation|GetActorRotation)) true true)
          (if (Variables|Default|GetTurnNormal?)
            (Audio|PlaySoundatLocation "/Game/Audio/Sound/sound/common/SE_Ringbooster.SE_Ringbooster" _returnvalue_2 "0, 0, 0" 1.0 1.0 0.0 "/Game/Audio/Sound/SoundAttenuation.SoundAttenuation" 0 0 :!label _label)
            (Effects|SpawnEmitteratLocation "/Game/Effects/Particles/P_DashringLaunch.P_DashringLaunch" (.location _returnvalue_3) (.rotation _returnvalue_3) (* (.scale _returnvalue_3) 1.5))
            (Utilities|FlowControl|Sequence
              (:then_0
                (bind _assonic_character_blueprint_2 (Utilities|Casting|CastToSonicCharacterBlueprint OtherActor))
                (Variables|/Game/Characters/Sonic/Blueprints/SonicCharacterBlueprint.SonicCharacterBlueprint_C|SetForceDisableInput? _assonic_character_blueprint_2 true)
                (Utilities|FlowControl|Delay (/ _inputdelay (Variables|/Script/Engine.Actor|GetCustomTimeDilation _assonic_character_blueprint_2)))
                (Variables|/Game/Characters/Sonic/Blueprints/SonicCharacterBlueprint.SonicCharacterBlueprint_C|SetForceDisableInput? _assonic_character_blueprint_2 false))
              (:then_1
                (bind _asshadow_character_blueprint (Utilities|Casting|CastToShadowCharacterBlueprint OtherActor))
                (Variables|/Game/Characters/Shadow/Blueprints/ShadowCharacterBlueprint.ShadowCharacterBlueprint_C|SetForceDisableInput? _asshadow_character_blueprint true)
                (Utilities|FlowControl|Delay (/ _inputdelay (Variables|/Script/Engine.Actor|GetCustomTimeDilation _asshadow_character_blueprint)))
                (Variables|/Game/Characters/Shadow/Blueprints/ShadowCharacterBlueprint.ShadowCharacterBlueprint_C|SetForceDisableInput? _asshadow_character_blueprint false)))
            (else
              (Default|CharacterVoices/Trick _assonic_character_blueprint))))
        (:then_1
          (Utilities|FlowControl|DoOnce false
            (:Completed
              (Default|AddScore _assonic_character_blueprint 1000 2e+01)
              (Variables|Default|SetTurnNormal? true :!label _label_2)
              (Audio|PlaySoundatLocation "/Game/Audio/Sound/sound/common/SE_Rainbowring.SE_Rainbowring" _returnvalue_2 "0, 0, 0" 1.0 1.0 0.0 "/Game/Audio/Sound/SoundAttenuation.SoundAttenuation" 0 0)
              (Effects|SpawnEmitteratLocation "/Game/Effects/Particles/P_TrickRamp.P_TrickRamp" _returnvalue_2 "0, 0, 0" (.scale _returnvalue))
              (Effects|SpawnEmitteratLocation "/Game/Effects/Particles/P_DashringLaunchRainbow.P_DashringLaunchRainbow" (.location _returnvalue) (.rotation _returnvalue) (* (.scale _returnvalue) 1.5))
              (Utilities|FlowControl|Sequence
                (:then_0
                  (Utilities|FlowControl|Delay 0.25)
                  (Class|SkinnedMeshComponent|SetSkeletalMesh _skeletalmesh "/Game/Blueprints/Objects/Assets/DashRings/Hoop.Hoop" true)
                  (Components|Animation|PlayAnimation _skeletalmesh "/Game/Blueprints/Objects/Assets/DashRings/Hoop_Anim.Hoop_Anim" true))))))))
    (:then_1
      (bind _asshadow_character_blueprint_2 (Utilities|Casting|CastToShadowCharacterBlueprint OtherActor))
      (Utilities|FlowControl|Sequence
        (:then_0
          (Variables|/Game/Characters/Shadow/Blueprints/ShadowCharacterBlueprint.ShadowCharacterBlueprint_C|SetIsStomping? _asshadow_character_blueprint_2 false)
          (Transformation|SetWorldLocation (Variables|/Script/Engine.Actor|GetRootComponent _asshadow_character_blueprint_2) (Transformation|GetActorLocation) false false)
          (Character|LaunchCharacter _asshadow_character_blueprint_2 (Math|Vector|RotateVector (+ (Transformation|GetActorForwardVector) (Math|Vector|MakeVector (Variables|Default|GetDashRingPower) 0.0 0.0)) (Transformation|GetActorRotation)) true true)
          (if (Variables|Default|GetTurnNormal?)
            (goto _label)
            (else
              (Default|CharacterVoices/Trick _asshadow_character_blueprint_2))))
        (:then_1
          (Utilities|FlowControl|DoOnce false
            (:Completed
              (Default|AddScore _asshadow_character_blueprint_2 1000 2e+01)
              (goto _label_2))))))))

(fn ConstructionScript
  (Transformation|SetWorldScale3D (Variables|Default|GetArrow) (Math|Vector|MakeVector (/ (/ (Variables|Default|GetDashRingPower) 1e+02) 3.0) 1.0 1.0)))