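; Dropped ring pickup that scatters from its instigating Sonic or Shadow player and can be re-collected briefly before vanishing.
; BeginPlay launches the physics sphere up, behind and away from that player, then timed delays enable pickup, start flickering and destroy it.
; Tick spins the ring and toggles visibility while fading.
; Overlap awards ring, score and boost to either character, with sound and particles that differ during Lightspeed Dash.
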(event EventBeginPlay
  (bind _id (Variables|Default|GetID))
  (bind _returnvalue (Game|GetPlayerCharacter _id))
  (|Getplayer)
  (Physics|SetPhysicsLinearVelocity (Variables|Default|GetSphere) (+ (* (Transformation|GetActorForwardVector _returnvalue) -3e+02) (* (Transformation|GetActorUpVector _returnvalue) 4.5e+02) (* (- (Transformation|GetActorLocation _returnvalue) (Transformation|GetActorLocation)) -2.0)) false "None")
  (Utilities|FlowControl|Delay 1.0)
  (Variables|Default|SetObtainable? true)
  (Utilities|FlowControl|Delay 2.0)
  (Variables|Default|SetFade? true)
  (Utilities|FlowControl|Delay 2.0)
  (Actor|DestroyActor))

(event Collision|EventActorBeginOverlap
  (params (OtherActor :type Actor%20Object%20Reference))
  (bind _returnvalue (Transformation|GetActorLocation))
  (bind _returnvalue_2 (Transformation|GetActorLocation))
  (bind _id (Variables|Default|GetID))
  (bind _returnvalue_3 (Game|GetPlayerCharacter _id))
  (bind _returnvalue_4 (Transformation|GetActorLocation _returnvalue_3))
  (bind _returnvalue_5 (- _returnvalue _returnvalue_4))
  (bind _returnvalue_6 (Math|Conversions|RotationFromXVector _returnvalue_5))
  (if (Variables|Default|GetObtainable?)
    (Utilities|FlowControl|Sequence
      (:then_0
        (bind _assonic_character_blueprint (Utilities|Casting|CastToSonicCharacterBlueprint OtherActor))
        (Default|AddRing _assonic_character_blueprint 1 100 1.0)
        (Utilities|FlowControl|Sequence
          (:then_0
            (|CollapseGraph_0_2_2 _assonic_character_blueprint _assonic_character_blueprint))
          (:then_1
            (if (Variables|/Game/Characters/Sonic/Blueprints/SonicCharacterBlueprint.SonicCharacterBlueprint_C|GetIsLightspeedDashing? _assonic_character_blueprint)
              (Effects|SpawnEmitteratLocation "/Game/Effects/Particles/P_AfterImageSonic.P_AfterImageSonic" _returnvalue_4 _returnvalue_6)
              (Effects|SpawnEmitterAttached "/Game/Effects/Particles/P_BoostRemove1.P_BoostRemove1" (Variables|/Script/Engine.Character|GetMesh _assonic_character_blueprint) "None" "0,85.000000,50.000000")
              (else
                (Effects|SpawnEmitteratLocation "/Game/Effects/Particles/P_RingGet.P_RingGet" _returnvalue_2 :!label _label)))
            (Audio|PlaySoundatLocation "/Game/Audio/Sound/sound/common/SE_Ring_Mix.SE_Ring_Mix" _returnvalue_2 "0, 0, 0" 0.5 1.0 0.0 "/Game/Audio/Sound/SoundAttenuation.SoundAttenuation" 0 0 :!label _label_2)
            (Actor|DestroyActor))))
      (:then_1
        (bind _asshadow_character_blueprint (Utilities|Casting|CastToShadowCharacterBlueprint OtherActor))
        (Default|AddRing _asshadow_character_blueprint 1 100 1.0)
        (if (Variables|/Game/Characters/Shadow/Blueprints/ShadowCharacterBlueprint.ShadowCharacterBlueprint_C|GetIsLightspeedDashing? _asshadow_character_blueprint)
          (Effects|SpawnEmitteratLocation "/Game/Effects/Particles/P_AfterImageShadow.P_AfterImageShadow" _returnvalue_4 _returnvalue_6)
          (Effects|SpawnEmitterAttached "/Game/Effects/Particles/P_BoostRemoveSH1.P_BoostRemoveSH1" (Variables|/Script/Engine.Character|GetMesh _asshadow_character_blueprint) "None" "0,85.000000,60.000000")
          (goto _label_2)
          (else
            (goto _label)))))))

(event EventTick
  (params (DeltaSeconds :type Float%20%28single-precision%29))
  (bind _returnvalue (Transformation|GetActorRotation))
  (bind (_roll _pitch _yaw) (Math|Rotator|BreakRotator _returnvalue))
  (Utilities|FlowControl|Sequence
    (:then_0
      (if (Variables|Default|GetFade?)
        (Utilities|FlowControl|Delay 0.1)
        (Rendering|ToggleVisibility (Variables|Default|GetSRing) false)))
    (:then_1
      (Transformation|SetActorRotation (Math|Rotator|MakeRotator _roll _pitch (+ _yaw 2.5))))))

(fn ConstructionScript)