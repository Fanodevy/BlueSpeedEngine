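; Underwater air bubble that periodically appears, rises and refills the breath of Sonic or Shadow characters.
; Tick runs chained Delays to toggle sphere overlap and visibility state, resetting and raising the sphere with a DoOnce-spawned attached emitter and sound.
; On overlap, per-character checks clear jump balls and play a breath montage, then falling players get full breath and a launch.
; Stomping, homing, lightspeed-dashing or boosting players pop the bubble instead.
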(event EventBeginPlay
  (Collision|SetCollisionResponsetoAllChannels (Variables|Default|GetSphere) "ECR_Ignore"))

(event Collision|EventActorBeginOverlap
  (params (OtherActor :type Actor%20Object%20Reference))
  (Utilities|FlowControl|Sequence
    (:then_0
      (bind _asshadow_character_blueprint (Utilities|Casting|CastToShadowCharacterBlueprint OtherActor))
      (Variables|Default|SetPlayer%20ID (Variables|/Game/Characters/Shadow/Blueprints/ShadowCharacterBlueprint.ShadowCharacterBlueprint_C|GetOwnerPlayerId _asshadow_character_blueprint))
      (|AssetCheck/Play _asshadow_character_blueprint _asshadow_character_blueprint _asshadow_character_blueprint
        (:then
          (if (AI|Components|NavMovement|IsFalling (Variables|/Script/Engine.Character|GetCharacterMovement (Game|GetPlayerCharacter (Variables|Default|GetPlayer%20ID))))
            (Variables|/Game/Characters/Shadow/Blueprints/ShadowCharacterBlueprint.ShadowCharacterBlueprint_C|SetPlayerBreathTotal _asshadow_character_blueprint 1e+02)
            (Character|LaunchCharacter (Game|GetPlayerCharacter (Variables|Default|GetPlayer%20ID)) (Math|Vector|MakeVector (.x (/ (Transformation|GetVelocity (Game|GetPlayerCharacter (Variables|Default|GetPlayer%20ID))) (Variables|Default|GetPlayerXYVelocityDivide))) (.y (/ (Transformation|GetVelocity (Game|GetPlayerCharacter (Variables|Default|GetPlayer%20ID))) (Variables|Default|GetPlayerXYVelocityDivide))) (Variables|Default|GetPlayerZLaunch%20Velocity)) true true :!label _label)
            (Utilities|IsValid (stale EventTick _returnvalue)
              (:Is%20Valid
                (Components|DestroyComponent (stale EventTick _returnvalue)))
              (:Is%20Not%20Valid
                _))
            (Audio|PlaySoundatLocation "/Game/Audio/Sound/sound/player/sn_water_breath.sn_water_breath" (Transformation|GetActorLocation (Game|GetPlayerCharacter (Variables|Default|GetPlayer%20ID))) "0, 0, 0" 1.0 1.0 0.0 "/Game/Audio/Sound/SoundAttenuation.SoundAttenuation" 0 0)
            (Effects|SpawnEmitteratLocation "/Game/Effects/Particles/P_UWBubbleGetA.P_UWBubbleGetA" (Transformation|GetWorldLocation (Variables|Default|GetSphere)) "0, 0, 0" "2.000000,2.000000,2.000000")
            (Collision|SetCollisionResponsetoAllChannels (Variables|Default|GetSphere) "ECR_Ignore")))
        (:else
          (Utilities|IsValid (stale EventTick _returnvalue) :!label _label_2
            (:Is%20Valid
              (Components|DestroyComponent (stale EventTick _returnvalue))
              (Effects|SpawnEmitteratLocation "/Game/Effects/Particles/P_UWBubblePop.P_UWBubblePop" (Transformation|GetActorLocation (Game|GetPlayerCharacter (Variables|Default|GetPlayer%20ID)))))))))
    (:then_1
      (bind _assonic_character_blueprint (Utilities|Casting|CastToSonicCharacterBlueprint OtherActor))
      (Variables|Default|SetPlayer%20ID (Variables|/Game/Characters/Sonic/Blueprints/SonicCharacterBlueprint.SonicCharacterBlueprint_C|GetOwnerPlayerId _assonic_character_blueprint))
      (|CollapseGraph_0 _assonic_character_blueprint _assonic_character_blueprint _assonic_character_blueprint
        (:execute
          (if (AI|Components|NavMovement|IsFalling (Variables|/Script/Engine.Character|GetCharacterMovement (Game|GetPlayerCharacter (Variables|Default|GetPlayer%20ID))))
            (Variables|/Game/Characters/Sonic/Blueprints/SonicCharacterBlueprint.SonicCharacterBlueprint_C|SetPlayerBreathTotal _assonic_character_blueprint 1e+02)
            (goto _label)))
        (:else
          (goto _label_2))))))

(event EventTick
  (params (DeltaSeconds :type Float%20%28single-precision%29))
  (bind _sphere (Variables|Default|GetSphere))
  (bind _sphere_2 (Variables|Default|GetSphere))
  (bind _relativelocation (Variables|/Script/Engine.SceneComponent|GetRelativeLocation _sphere_2))
  (bind (_x _y) (Math|Vector|BreakVector _relativelocation))
  (Utilities|FlowControl|Sequence
    (:then_0
      (Utilities|FlowControl|Delay (Variables|Default|GetBubbleShowUpTime))
      (Variables|Default|SetBubbleShowUp? true)
      (Collision|SetCollisionResponsetoAllChannels (Variables|Default|GetSphere) "ECR_Overlap")
      (Utilities|FlowControl|Delay (Variables|Default|GetBubbleDisappearTime))
      (Collision|SetCollisionResponsetoAllChannels (Variables|Default|GetSphere) "ECR_Ignore")
      (Variables|Default|SetBubbleShowUp? false))
    (:then_1
      (if (Variables|Default|GetBubbleShowUp?)
        (Transformation|SetRelativeLocation _sphere_2 (Math|Interpolation|VInterpTo _relativelocation (Math|Vector|MakeVector _x _y 5e+02) DeltaSeconds 1.0) false false)
        (Utilities|FlowControl|DoOnce false :!label _label
          (:Completed
            (bind _returnvalue (Effects|SpawnEmitterAttached "/Game/Effects/Particles/P_UWBubbleGet.P_UWBubbleGet" _sphere "None"))
            (Transformation|SetRelativeLocation _sphere "0, 0, 0" false false)
            (Audio|PlaySoundatLocation "/Game/Audio/Sound/sound/common/SE_Bubble_01.SE_Bubble_01" (Transformation|GetWorldLocation _sphere) "0, 0, 0" 0.25 1.0 0.0 "/Game/Audio/Sound/SoundAttenuation.SoundAttenuation" 0 0)))
        (else
          (goto _label Reset))))))

(fn ConstructionScript)