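; Checkpoint gate that fires once when Sonic or Shadow crosses it, setting both players' multiplayer respawn transforms and saving progress.
; It writes the respawn point to the "temp1" TempSave slot, along with snapshots of listed actor classes such as balloons, GUN enemies and capsules.
; Posts play speed-scaled montages with sound, particles and light changes, plus slow motion at very high speed.
; The construction script sizes the gate from CheckpointWidth.
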(event OnComponentBeginOverlap(Middle)
  (params (OverlappedComponent :type Primitive%20Component%20Object%20Reference) (OtherActor :type Actor%20Object%20Reference) (OtherComp :type Primitive%20Component%20Object%20Reference) (OtherBodyIndex :type Integer) (bFromSweep :type Boolean) (SweepResult :type Hit%20Result%20Structure%20%28by%20ref%29))
  (bind _returnvalue (Transformation|GetActorLocation))
  (bind _returnvalue_2 (Transformation|GetActorRotation))
  (bind _returnvalue_3 (Game|GetPlayerCharacter 0))
  (bind _returnvalue_4 (Transformation|GetVelocity _returnvalue_3))
  (bind _returnvalue_5 (Math|Vector|VectorLength _returnvalue_4))
  (bind _returnvalue_6 (/ _returnvalue_5 2.5e+03))
  (bind _returnvalue_7 (Math|Float|Clamp(Float) _returnvalue_6 1.0 1e+04))
  (Utilities|FlowControl|Sequence
    (:then_0
      (bind _assonic_character_blueprint (Utilities|Casting|CastToSonicCharacterBlueprint OtherActor))
      (Variables|Default|SetSonic _assonic_character_blueprint))
    (:then_1
      (bind _asshadow_character_blueprint (Utilities|Casting|CastToShadowCharacterBlueprint OtherActor))
      (Variables|Default|SetShadow _asshadow_character_blueprint)))
  (Utilities|FlowControl|DoOnce false
    (:Completed
      (Utilities|FlowControl|Sequence
        (:then_0
          (Variables|Default|SetCheckLoc (+ _returnvalue "0, 0,2.000000"))
          (Variables|Default|SetCheckRot (Math|Rotator|MakeRotator (.roll _returnvalue_2) (.pitch _returnvalue_2) (+ (.yaw _returnvalue_2) 9e+01)))
          (|SetforMultiplayer
            (:execute
              (bind _returnvalue_8 (SaveGame|DoesSaveGameExist "temp1"))
              (if _returnvalue_8
                (bind _returnvalue_9 (SaveGame|LoadGamefromSlot "temp1"))
                (bind _output_get (Variables|Default|SetSaverSubclass _returnvalue_9))
                (bind _astemp_save (Utilities|Casting|CastToTempSave _output_get))
                (Utilities|Array|Clear (Variables|/Game/Blueprints/Data/Save/TempSave.TempSave_C|GetNoPropActors _astemp_save))
                (Utilities|Array|Clear (Variables|/Game/Blueprints/Data/Save/TempSave.TempSave_C|GetBalloonActors _astemp_save))
                (Utilities|Array|Clear (Variables|/Game/Blueprints/Data/Save/TempSave.TempSave_C|GetGUNEnemyActors _astemp_save))
                (Utilities|FlowControl|Sequence
                  (:then_0
                    ;[1 1 1] Player
                    (Variables|/Game/Blueprints/Data/Save/TempSave.TempSave_C|SetSavePlyrLoc _astemp_save (Variables|Default|GetCheckLoc))
                    (Variables|/Game/Blueprints/Data/Save/TempSave.TempSave_C|SetSavePlyrRot _astemp_save (Variables|Default|GetCheckRot)))
                  (:then_1
                    ;[1 1 1] Other Actors
                    (CallFunction|SaveActorPositionandClass (Variables|/Game/Blueprints/Data/Save/TempSave.TempSave_C|GetSavedNoPropActors _astemp_save) (Variables|/Game/Blueprints/Data/Save/TempSave.TempSave_C|GetNoPropActors _astemp_save) (Variables|/Game/Blueprints/Data/Save/TempSave.TempSave_C|GetSavedBaloonActors _astemp_save) (Variables|/Game/Blueprints/Data/Save/TempSave.TempSave_C|GetBalloonActors _astemp_save) (Variables|/Game/Blueprints/Data/Save/TempSave.TempSave_C|GetSavedGUN%20EnemyActors _astemp_save) (Variables|/Game/Blueprints/Data/Save/TempSave.TempSave_C|GetGUNEnemyActors _astemp_save) (Variables|/Game/Blueprints/Data/Save/TempSave.TempSave_C|GetSavedRingCapsuleActors _astemp_save) (Variables|/Game/Blueprints/Data/Save/TempSave.TempSave_C|GetRingCapsuleActors _astemp_save))))
                (else
                  (bind _returnvalue_10 (SaveGame|CreateSaveGameObject "/Game/Blueprints/Data/Save/TempSave.TempSave_C"))
                  (bind _output_get_2 (Variables|Default|SetSaverSubclass _returnvalue_10))
                  (bind _astemp_save_2 (Utilities|Casting|CastToTempSave _output_get_2))
                  (Utilities|FlowControl|Sequence
                    (:then_0
                      (Variables|/Game/Blueprints/Data/Save/TempSave.TempSave_C|SetSavePlyrLoc _astemp_save_2 (Variables|Default|GetCheckLoc))
                      (Variables|/Game/Blueprints/Data/Save/TempSave.TempSave_C|SetSavePlyrRot _astemp_save_2 (Variables|Default|GetCheckRot)))
                    (:then_1
                      (CallFunction|SaveActorPositionandClass (Variables|/Game/Blueprints/Data/Save/TempSave.TempSave_C|GetSavedNoPropActors _astemp_save_2) (Variables|/Game/Blueprints/Data/Save/TempSave.TempSave_C|GetNoPropActors _astemp_save_2) (Variables|/Game/Blueprints/Data/Save/TempSave.TempSave_C|GetSavedBaloonActors _astemp_save_2) (Variables|/Game/Blueprints/Data/Save/TempSave.TempSave_C|GetBalloonActors _astemp_save_2) (Variables|/Game/Blueprints/Data/Save/TempSave.TempSave_C|GetSavedGUN%20EnemyActors _astemp_save_2) (Variables|/Game/Blueprints/Data/Save/TempSave.TempSave_C|GetGUNEnemyActors _astemp_save_2) (Variables|/Game/Blueprints/Data/Save/TempSave.TempSave_C|GetSavedRingCapsuleActors _astemp_save_2) (Variables|/Game/Blueprints/Data/Save/TempSave.TempSave_C|GetRingCapsuleActors _astemp_save_2))))))
              (bind _returnvalue_11 (SaveGame|SaveGametoSlot (Variables|Default|GetSaverSubclass) "temp1"))
              (Development|PrintString "CP Reached" _returnvalue_11 false))))
        (:then_1
          (Audio|PlaySoundatLocation "/Game/Audio/Sound/sound/common/SE_Checkpoint.SE_Checkpoint" _returnvalue "0, 0, 0" 1.0 1.0 0.0 "/Game/Audio/Sound/SoundAttenuation.SoundAttenuation" 0 0)
          (Animation|Montage|PlayMontage (Variables|Default|GetSkeletalMesh) "/Game/Blueprints/Objects/Assets/Checkpoint/Left/cmn_obj_pointmarkerL_HD_skl_Montage.cmn_obj_pointmarkerL_HD_skl_Montage" _returnvalue_7
            (:then
              (Animation|Montage|PlayMontage (Variables|Default|GetSkeletalMesh1) "/Game/Blueprints/Objects/Assets/Checkpoint/Right/cmn_obj_pointmarkerR_HD_skl_Montage.cmn_obj_pointmarkerR_HD_skl_Montage" _returnvalue_7
                (:then
                  (Effects|SpawnEmitterAttached "/Game/Effects/Particles/P_CheckpointGlitter.P_CheckpointGlitter" (Variables|Default|GetSkeletalMesh) "effectpointL" "0, 0, 0" "0, 0, 0" "1.000000,1.000000,1.000000" "SnapToTarget")
                  (Effects|SpawnEmitterAttached "/Game/Effects/Particles/P_CheckpointGlitter.P_CheckpointGlitter" (Variables|Default|GetSkeletalMesh1) "effectpointR" "0,-0.300000,0.000000" "0, 0, 0" "1.000000,1.000000,1.000000" "SnapToTarget")
                  (Rendering|SetVisibility (Variables|Default|GetPlane) false false)
                  (Effects|SpawnEmitteratLocation "/Game/Effects/Particles/P_CheckpointCross.P_CheckpointCross" (+ (Transformation|GetWorldLocation (Variables|Default|GetMiddle)) "0, 0,30.000000") "0, 0, 0" "2.000000,2.000000,2.000000")
                  (if (> (Math|Vector|VectorLength (Transformation|GetVelocity (Game|GetPlayerCharacter 0))) 7e+03)
                    (Utilities|FlowControl|Sequence
                      (:then_0
                        (Utilities|IsValid (Variables|Default|GetShadow)
                          (:Is%20Valid
                            (Default|SlowMotion (Variables|Default|GetShadow) 0.04))))
                      (:then_1
                        (Utilities|IsValid (Variables|Default|GetSonic)
                          (:Is%20Valid
                            (Default|SlowMotion (Variables|Default|GetSonic) 0.04)))))))
                (:OnCompleted
                  (Rendering|Material|SetMaterial (Variables|Default|GetSkeletalMesh1) 4 "/Game/Blueprints/Objects/Assets/Checkpoint/Left/cmn_obj_pointlaser_mat_laserpos_lumi1.cmn_obj_pointlaser_mat_laserpos_lumi1")
                  (Effects|SpawnEmitterAttached "/Game/Effects/Particles/P_CheckpointBulb.P_CheckpointBulb" (Variables|Default|GetSkeletalMesh) "effectpointL" "0, 0, 0" "0, 0, 0" "1.000000,1.000000,1.000000" "SnapToTarget" :!label _label)
                  (Effects|SpawnEmitterAttached "/Game/Effects/Particles/P_CheckpointBulb.P_CheckpointBulb" (Variables|Default|GetSkeletalMesh1) "effectpointR" "0,-0.300000,0.000000" "0, 0, 0" "1.000000,1.000000,1.000000" "SnapToTarget")
                  (Rendering|Components|Light|SetLightColor (Variables|Default|GetPointLight) "(R=1.000000,G=0.672443,B=0.000000,A=1.000000)" true))))
            (:OnCompleted
              (Rendering|Material|SetMaterial (Variables|Default|GetSkeletalMesh) 4 "/Game/Blueprints/Objects/Assets/Checkpoint/Left/cmn_obj_pointlaser_mat_laserpos_lumi1.cmn_obj_pointlaser_mat_laserpos_lumi1")
              (goto _label))))))))

(event EventBeginPlay)

(event Collision|EventActorBeginOverlap
  (params (OtherActor :type Actor%20Object%20Reference)))

(fn ConstructionScript
  (bind _checkpointwidth (Variables|Default|GetCheckpointWidth))
  (Transformation|SetRelativeLocation (Variables|Default|GetLeftSide) (Math|Vector|MakeVector (* _checkpointwidth -1.0) 0.0 5e+01) false false)
  (Transformation|SetRelativeLocation (Variables|Default|GetRightSide) (Math|Vector|MakeVector _checkpointwidth 0.0 5e+01) false false)
  (Transformation|SetWorldScale3D (Variables|Default|GetMiddle) (Math|Vector|MakeVector (* (/ _checkpointwidth 1.5e+02) 1.2) 1.0 1.0))
  (Transformation|AttachComponentToComponent (Variables|Default|GetPointLight2) (Variables|Default|GetSkeletalMesh) "effectpointL" "KeepRelative" "KeepRelative" "KeepRelative" true)
  (Transformation|AttachComponentToComponent (Variables|Default|GetPointLight3) (Variables|Default|GetSkeletalMesh1) "effectpointR" "KeepRelative" "KeepRelative" "KeepRelative" true))

(fn SaveActorPositionandClass
  (params (ArrayOther :type Array%20of%20Actor%20Class%20References) (TargetArrayOther :type Array%20of%20No%20Prop%20Actors%20Structures) (ArrayBaloons :type Array%20of%20Actor%20Class%20References) (TargetArrayBaloons :type Array%20of%20Baloon%20Actors%20Structures) (ArrayGUN :type Array%20of%20Actor%20Class%20References) (TargetArrayGUN :type Array%20of%20GUN%20Enemy%20Actors%20Structures) (ArrayRingCapsule :type Array%20of%20Actor%20Class%20References) (TargetArrayRingCapsule :type Array%20of%20Ring%20Capsule%20Actor%20Structures))
  ;[1 1 1] Rings etc.
  (for _array_element ArrayOther
    (bind _outactors (Actor|GetAllActorsOfClass _array_element))
    (for _array_element_2 _outactors
      (Utilities|Array|Add TargetArrayOther (Utilities|Struct|MakeNoPropActors _array_element (Transformation|GetActorTransform _array_element_2)))))
  ;[1 1 1] Baloons
  (for _array_element_3 ArrayBaloons
    (bind _outactors_2 (Actor|GetAllActorsOfClass _array_element_3))
    (for _array_element_4 _outactors_2
      (bind _asballoon (Utilities|Casting|CastToBalloon _array_element_4))
      (Utilities|Array|Add TargetArrayBaloons (Utilities|Struct|MakeBaloonActors _array_element_3 (Transformation|GetActorTransform _array_element_4) (Variables|/Game/Blueprints/Objects/Balloon.Balloon_C|GetBalloonColor _asballoon) (Variables|/Game/Blueprints/Objects/Balloon.Balloon_C|GetBoostEnergyAmount _asballoon)))))
  ;[1 1 1] GUN Bots
  (for _array_element_5 ArrayGUN
    (bind _outactors_3 (Actor|GetAllActorsOfClass _array_element_5))
    (for _array_element_6 _outactors_3
      (Utilities|FlowControl|Sequence
        (:then_0
          (bind _asgunmono_beetle (Utilities|Casting|CastToGUNMonoBeetle _array_element_6))
          (Utilities|Array|Add TargetArrayGUN (Utilities|Struct|MakeGUNEnemyActors _array_element_5 (Transformation|GetActorTransform _array_element_6) (Variables|/Game/Enemies/GUNMonoBeetle.GUNMonoBeetle_C|GetEnemyRadius _asgunmono_beetle) 0.0 0.0 (Variables|/Game/Enemies/GUNMonoBeetle.GUNMonoBeetle_C|GetScoreAmount _asgunmono_beetle) (Variables|/Game/Enemies/GUNMonoBeetle.GUNMonoBeetle_C|GetBoostEnergyAmount _asgunmono_beetle) (Variables|/Game/Enemies/GUNMonoBeetle.GUNMonoBeetle_C|GetDustRange _asgunmono_beetle))))
        (:then_1
          (bind _asgunbeetle (Utilities|Casting|CastToGUNBeetle _array_element_6))
          (Utilities|Array|Add TargetArrayGUN (Utilities|Struct|MakeGUNEnemyActors _array_element_5 (Transformation|GetActorTransform _array_element_6) (Variables|/Game/Enemies/GUNBeetle.GUNBeetle_C|GetEnemyRadius _asgunbeetle) (Variables|/Game/Enemies/GUNBeetle.GUNBeetle_C|GetChargeTime _asgunbeetle) (Variables|/Game/Enemies/GUNBeetle.GUNBeetle_C|GetShotCoolDown _asgunbeetle) (Variables|/Game/Enemies/GUNBeetle.GUNBeetle_C|GetScoreAmount _asgunbeetle) (Variables|/Game/Enemies/GUNBeetle.GUNBeetle_C|GetBoostEnergyAmount _asgunbeetle) (Variables|/Game/Enemies/GUNBeetle.GUNBeetle_C|GetDustRange _asgunbeetle))))
        (:then_2
          (bind _asgunhunter (Utilities|Casting|CastToGUNHunter _array_element_6))
          (Utilities|Array|Add TargetArrayGUN (Utilities|Struct|MakeGUNEnemyActors _array_element_5 (Transformation|GetActorTransform _array_element_6) (Variables|/Game/Enemies/GUNHunter.GUNHunter_C|GetEnemyRadius _asgunhunter) (Variables|/Game/Enemies/GUNHunter.GUNHunter_C|GetChargeTime _asgunhunter) (Variables|/Game/Enemies/GUNHunter.GUNHunter_C|GetShotCoolDown _asgunhunter) (Variables|/Game/Enemies/GUNHunter.GUNHunter_C|GetScoreAmount _asgunhunter) (Variables|/Game/Enemies/GUNHunter.GUNHunter_C|GetBoostEnergyAmount _asgunhunter) (Variables|/Game/Enemies/GUNHunter.GUNHunter_C|GetDustRange _asgunhunter))))
        (:then_3
          (bind _asgold_beetle (Utilities|Casting|CastToGoldBeetle _array_element_6))
          (Utilities|Array|Add TargetArrayGUN (Utilities|Struct|MakeGUNEnemyActors _array_element_5 (Transformation|GetActorTransform _array_element_6) (Variables|/Game/Enemies/GoldBeetle.GoldBeetle_C|GetEnemyRadius _asgold_beetle) 0.0 0.0 (Variables|/Game/Enemies/GoldBeetle.GoldBeetle_C|GetScoreAmount _asgold_beetle) (Variables|/Game/Enemies/GoldBeetle.GoldBeetle_C|GetBoostEnergyAmount _asgold_beetle) (Variables|/Game/Enemies/GoldBeetle.GoldBeetle_C|GetDustRange _asgold_beetle)))))))
  ;[1 1 1] Ring capsule/ Egg Capsule
  (for _array_element_7 ArrayRingCapsule
    (bind _outactors_4 (Actor|GetAllActorsOfClass _array_element_7))
    (for _array_element_8 _outactors_4
      (Utilities|FlowControl|Sequence
        (:then_0
          (bind _asring_capsule (Utilities|Casting|CastToRingCapsule _array_element_8))
          (Utilities|Array|Add TargetArrayRingCapsule (Utilities|Struct|MakeRingCapsuleActor _array_element_7 (Transformation|GetActorTransform _array_element_8) (Variables|/Game/Blueprints/Objects/RingCapsule.RingCapsule_C|GetRingamount _asring_capsule))))
        (:then_1
          (bind _asegg_capsule (Utilities|Casting|CastToEggCapsule _array_element_8))
          (Utilities|Array|Add TargetArrayRingCapsule (Utilities|Struct|MakeRingCapsuleActor _array_element_7 (Transformation|GetActorTransform _array_element_8) (Variables|/Game/Blueprints/Objects/EggCapsule.EggCapsule_C|GetRingAmount _asegg_capsule))))))))